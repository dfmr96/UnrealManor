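; BP_AudioManager is a level actor that switches the background music as the first-person player moves between the East Wing, West Wing and Main Hall.
; Each area has an overlap component whose begin-overlap event confirms that the overlapping actor is the player character.
; It then assigns that area's BGM track to the single shared Audio component and plays it from the start, with no crossfade or check for an already-playing track.
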(event OnComponentBeginOverlap(EastWing)
  (params (OverlappedComponent :type Primitive%20Component%20Object%20Reference) (OtherActor :type Actor%20Object%20Reference) (OtherComp :type Primitive%20Component%20Object%20Reference) (OtherBodyIndex :type Integer) (bFromSweep :type Boolean) (SweepResult :type Hit%20Result%20Structure%20%28by%20ref%29))
  (bind _audio (Variables|Default|GetAudio))
  (if (== (.AsBP%20First%20Person%20Character (Utilities|Casting|CastToBP_FirstPersonCharacter (Game|GetPlayerCharacter 0))) OtherActor)
    (Audio|Components|Audio|SetSound _audio (Variables|Default|GetBGM1))
    (Audio|Components|Audio|Play _audio 0.0)))

(event OnComponentBeginOverlap(WestWing)
  (params (OverlappedComponent :type Primitive%20Component%20Object%20Reference) (OtherActor :type Actor%20Object%20Reference) (OtherComp :type Primitive%20Component%20Object%20Reference) (OtherBodyIndex :type Integer) (bFromSweep :type Boolean) (SweepResult :type Hit%20Result%20Structure%20%28by%20ref%29))
  (bind _audio (Variables|Default|GetAudio))
  (if (== (.AsBP%20First%20Person%20Character (Utilities|Casting|CastToBP_FirstPersonCharacter (Game|GetPlayerCharacter 0))) OtherActor)
    (Audio|Components|Audio|SetSound _audio (Variables|Default|GetBGM1_0))
    (Audio|Components|Audio|Play _audio 0.0)))

(event OnComponentBeginOverlap(MainHall)
  (params (OverlappedComponent :type Primitive%20Component%20Object%20Reference) (OtherActor :type Actor%20Object%20Reference) (OtherComp :type Primitive%20Component%20Object%20Reference) (OtherBodyIndex :type Integer) (bFromSweep :type Boolean) (SweepResult :type Hit%20Result%20Structure%20%28by%20ref%29))
  (bind _audio (Variables|Default|GetAudio))
  (if (== (.AsBP%20First%20Person%20Character (Utilities|Casting|CastToBP_FirstPersonCharacter (Game|GetPlayerCharacter 0))) OtherActor)
    (Audio|Components|Audio|SetSound _audio (Variables|Default|GetBGM1_1))
    (Audio|Components|Audio|Play _audio 0.0)))

(event EventBeginPlay)

(event Collision|EventActorBeginOverlap
  (params (OtherActor :type Actor%20Object%20Reference)))

(event EventTick
  (params (DeltaSeconds :type Float%20%28single-precision%29)))

(fn ConstructionScript)