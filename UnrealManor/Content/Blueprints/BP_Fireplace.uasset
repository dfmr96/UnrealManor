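; BP_Fireplace is a puzzle fireplace that takes two inventory items in order and reveals a hidden key once lit.
; CheckItemUsed matches item row names, setting CubesPlaced first, then burning on the second item and showing hints for wrong items.
; Lighting sets PFire's time dilation to normal, plays audio, swaps Frame1's material and lets Visibility and Camera traces ignore the meshes.
; Interact shows the unburnt text through the player's TextPrompter.
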(event EventInteract
  (Default|WriteText (Variables|/Game/Core/FirstPerson/Blueprints/BP_FirstPersonCharacter.BP_FirstPersonCharacter_C|GetTextPrompter (.AsBP%20First%20Person%20Character (Utilities|Casting|CastToBP_FirstPersonCharacter (Game|GetPlayerCharacter 0)))) (Variables|Default|GetUnBurntText)))

(fn ConstructionScript)

(fn CheckItemUsed
  (params (ItemUsed :type Data%20Table%20Row%20Handle%20Structure))
  (bind _returnvalue (Game|GetPlayerCharacter 0))
  (bind _komin_low (Variables|Default|Getkomin_low))
  (bind _frame1 (Variables|Default|GetFrame1))
  (bind _asbp_first_person_character (Utilities|Casting|CastToBP_FirstPersonCharacter _returnvalue))
  (bind _textprompter (Variables|/Game/Core/FirstPerson/Blueprints/BP_FirstPersonCharacter.BP_FirstPersonCharacter_C|GetTextPrompter _asbp_first_person_character))
  (if (Variables|Default|GetcubesPlaced?)
    (if (== (.rowname ItemUsed) (.rowname (Variables|Default|GetItemRequired_2)))
      (Default|WriteText _textprompter (Variables|Default|GetBurningText))
      (Variables|Default|SetisBurnt? true)
      (Variables|/Script/Engine.ParticleSystemComponent|SetCustomTimeDilation (Variables|Default|GetP_Fire) 1.0)
      (Rendering|Material|SetMaterial _frame1 1 "/Engine/MaterialTemplates/PerfTricks/M_SpecularUsingDiffuse.M_SpecularUsingDiffuse")
      (Collision|SetCollisionResponsetoChannel _frame1 "ECC_Visibility" "ECR_Ignore")
      (Collision|SetCollisionResponsetoChannel _frame1 "ECC_Camera" "ECR_Ignore")
      (Collision|SetCollisionResponsetoChannel _komin_low "ECC_Visibility" "ECR_Ignore")
      (Collision|SetCollisionResponsetoChannel _komin_low "ECC_Camera" "ECR_Ignore")
      (Rendering|SetActorHiddenInGame (Variables|Default|GetKey) false)
      (Audio|Components|Audio|Play (Variables|Default|GetFireAudio) 0.0)
      (return true)
      (else
        (Default|WriteText _textprompter "I just need something to light the fireplace with")
        (return false)))
    (elif (== (.rowname ItemUsed) (.rowname (Variables|Default|GetItemRequired_1)))
      (Variables|Default|SetcubesPlaced? true)
      (return true)
      (elif (== (.rowname ItemUsed) (.rowname (Variables|Default|GetItemRequired_2)))
        (Default|WriteText _textprompter "I can't burn the wood yet, I need something else.")
        (else
          (Default|WriteText _textprompter "Can't use this item here")
          (return false))))))

(fn GetItemRequired
  (return ""))