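; Painting puzzle controller that removes a referenced object once four paintings all hold their correct codes.
; CheckCodes, which nothing in this Blueprint calls, compares each painting's CodeSubmitted to its expected code in nested order, stopping at the first mismatch.
; Each match immediately plays a confirmation sound; full success adds a delayed fire-stop sound, then destroys ObjectToDestroy if valid after another delay.
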(event Custom|CheckCodes
  (bind _objecttodestroy (Variables|Default|GetObjectToDestroy))
  (bind _output (Utilities|ResolveSoftReference _objecttodestroy))
  (if (== (Variables|/Game/Blueprints/Puzzles/Paintings/BP_Painting.BP_Painting_C|GetCodeSubmitted (Utilities|ResolveSoftReference (Variables|Default|GetPainting1))) (Variables|Default|GetPaintingCode_1))
    (Audio|PlaySound2D "/Game/Audio/A_ButtonOK.A_ButtonOK" 1.0 1.0 0.0 0 0)
    (if (== (Variables|/Game/Blueprints/Puzzles/Paintings/BP_Painting.BP_Painting_C|GetCodeSubmitted (Utilities|ResolveSoftReference (Variables|Default|GetPainting2))) (Variables|Default|GetPaintingCode_2))
      (Audio|PlaySound2D "/Game/Audio/A_ButtonOK.A_ButtonOK" 1.0 1.0 0.0 0 0)
      (if (== (Variables|/Game/Blueprints/Puzzles/Paintings/BP_Painting.BP_Painting_C|GetCodeSubmitted (Utilities|ResolveSoftReference (Variables|Default|GetPainting3))) (Variables|Default|GetPaintingCode_3))
        (Audio|PlaySound2D "/Game/Audio/A_ButtonOK.A_ButtonOK" 1.0 1.0 0.0 0 0)
        (if (== (Variables|/Game/Blueprints/Puzzles/Paintings/BP_Painting.BP_Painting_C|GetCodeSubmitted (Utilities|ResolveSoftReference (Variables|Default|GetPainting4))) (Variables|Default|GetPaintingCode_4))
          (Audio|PlaySound2D "/Game/Audio/A_ButtonOK.A_ButtonOK" 1.0 1.0 0.0 0 0)
          (Utilities|FlowControl|Delay 1.3)
          (Audio|PlaySound2D "/Game/Audio/A_FireStop.A_FireStop" 1.0 1.0 0.0 0 0)
          (Utilities|FlowControl|Delay 0.5)
          (Utilities|IsValid _output
            (:Is%20Valid
              (Actor|DestroyActor _output))))))))

(event EventBeginPlay)

(event Collision|EventActorBeginOverlap
  (params (OtherActor :type Actor%20Object%20Reference)))

(event EventTick
  (params (DeltaSeconds :type Float%20%28single-precision%29)))

(fn ConstructionScript)