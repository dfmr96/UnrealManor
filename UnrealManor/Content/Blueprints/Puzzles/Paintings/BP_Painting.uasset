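; A painting actor that forms one piece of a multi-painting code puzzle.
; SubmitCode writes the entered code into the referenced PaintingPuzzle's SubmittedCodes array at this painting's PaintingID, then debug-prints the expected code.
; On a match it plays a confirmation sound and calls CheckCodes on the puzzle; a wrong code stays stored without triggering that check.
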(event EventBeginPlay)

(event Collision|EventActorBeginOverlap
  (params (OtherActor :type Actor%20Object%20Reference)))

(event EventTick
  (params (DeltaSeconds :type Float%20%28single-precision%29)))

(fn ConstructionScript)

(fn SubmitCode
  (params (codeSubmitted :type Integer))
  (bind _paintingid (Variables|Default|GetPaintingID))
  (bind _paintingpuzzle (Variables|Default|GetPaintingPuzzle))
  (bind _paintingcodes (Variables|/Game/Blueprints/Puzzles/Paintings/BP_PaintingPuzzle.BP_PaintingPuzzle_C|GetPaintingCodes _paintingpuzzle))
  (bind _output (Utilities|Array|Get(acopy) _paintingcodes _paintingid))
  (Utilities|Array|SetArrayElem (Variables|/Game/Blueprints/Puzzles/Paintings/BP_PaintingPuzzle.BP_PaintingPuzzle_C|GetSubmittedCodes (Variables|Default|GetPaintingPuzzle)) _paintingid codeSubmitted)
  (Development|PrintString (Utilities|String|ToString(Integer) _output))
  (if (== _output codeSubmitted)
    (Development|PrintString "Right code")
    (Audio|PlaySound2D "/Game/Audio/A_ButtonOK.A_ButtonOK" 1.0 1.0 0.0 0 0)
    (Default|CheckCodes (Variables|Default|GetPaintingPuzzle))))