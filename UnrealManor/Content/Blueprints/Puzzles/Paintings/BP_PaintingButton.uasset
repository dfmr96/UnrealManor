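; BP_PaintingButton is an interactable button in the painting puzzle that enters a code digit for its linked painting.
; On Interact it writes its CodeDigit to the painting's CodeSubmitted, then calls CheckCodes on that painting's PaintingPuzzle.
; A GetCode function exposes the button's digit.
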(event EventBeginPlay)

(event Collision|EventActorBeginOverlap
  (params (OtherActor :type Actor%20Object%20Reference)))

(event EventTick
  (params (DeltaSeconds :type Float%20%28single-precision%29)))

(event EventInteract
  (bind _painting (Variables|Default|GetPainting))
  (bind _output (Utilities|ResolveSoftReference _painting))
  (Development|PrintString "Button interacted")
  (Variables|/Game/Blueprints/Puzzles/Paintings/BP_Painting.BP_Painting_C|SetCodeSubmitted _output (Variables|Default|GetCodeDigit))
  (Default|CheckCodes (Utilities|ResolveSoftReference (Variables|/Game/Blueprints/Puzzles/Paintings/BP_Painting.BP_Painting_C|GetPaintingPuzzle _output))))

(fn ConstructionScript)

(fn GetCode
  (return (Variables|Default|GetCodeDigit)))