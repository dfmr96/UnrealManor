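; BP_DeerSkull is a deer skull puzzle that takes two gems as items and releases a key.
; CheckItemUsed looks up the used item in RequiredItems by row name, and the array index selects whether the blue or red gem becomes visible.
; Each placement increments a gem counter, and CheckGems disables the skull's collision and enables physics on the key once it reaches two.
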(event EventCheckItemUsed
  (params (ItemUsed :type Data%20Table%20Row%20Handle%20Structure))
  (bind (_array_element _array_index) (Utilities|Array|ForEachLoopwithBreak (Variables|Default|GetRequiredItems) :!label _label)
    (:LoopBody
      (if (== (.rowname ItemUsed) (.rowname _array_element))
        (goto _label Break)))
    (:Completed
      (if (== _array_index 0)
        (Rendering|SetVisibility (Variables|Default|GetBlueGem) true false)
        (Math|Integer|IncrementInt (Variables|Default|GetGems) :!label _label_2
          (:%20%20
            (CallFunction|CheckGems)))
        (elif (== _array_index 1)
          (Rendering|SetVisibility (Variables|Default|GetRedGem) true false)
          (goto _label_2))))))

(fn ConstructionScript)

(fn CheckGems
  (if (== (Variables|Default|GetGems) 2)
    (Collision|SetCollisionEnabled (Variables|Default|GetHirschschädel) "NoCollision")
    (Physics|SetSimulatePhysics (Variables|/Game/Blueprints/Inventory/ItemClasses/BP_GroundItem.BP_GroundItem_C|GetBody (Variables|Default|GetKey)) true)))

(fn GetItemRequired
  (return ""))