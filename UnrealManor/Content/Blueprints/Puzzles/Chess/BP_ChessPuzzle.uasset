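; BP_ChessPuzzle is a chess puzzle that moves a wall as its reward when pieces are placed on their target spots.
; Collision volumes for the white rook, white bishop and black rook adjust a counter on overlap begin and end, playing a click on arrival.
; CheckPieces triggers ShowReward at a count of six, although only three pieces are handled here.
; ShowReward adds audio and runs a timeline that offsets the wall's location each update.
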(event OnComponentBeginOverlap(WhiteRookCol)
  (params (OverlappedComponent :type Primitive%20Component%20Object%20Reference) (OtherActor :type Actor%20Object%20Reference) (OtherComp :type Primitive%20Component%20Object%20Reference) (OtherBodyIndex :type Integer) (bFromSweep :type Boolean) (SweepResult :type Hit%20Result%20Structure%20%28by%20ref%29))
  (if (== OtherActor (Variables|Default|GetWhiteRook))
    (Development|PrintString "WhiteRook on site")
    (Math|Integer|IncrementInt (Variables|Default|GetPiecesOnSite)
      (:%20%20
        (CallFunction|CheckPieces)
        (Audio|Components|Audio|Play (Variables|Default|Getmanhole-click-clack-41197) 0.0)))))

(event OnComponentBeginOverlap(WhiteBishopCol)
  (params (OverlappedComponent :type Primitive%20Component%20Object%20Reference) (OtherActor :type Actor%20Object%20Reference) (OtherComp :type Primitive%20Component%20Object%20Reference) (OtherBodyIndex :type Integer) (bFromSweep :type Boolean) (SweepResult :type Hit%20Result%20Structure%20%28by%20ref%29))
  (if (== OtherActor (Variables|Default|GetWhiteBishop))
    (Development|PrintString "White Bishop  on site")
    (Math|Integer|IncrementInt (Variables|Default|GetPiecesOnSite)
      (:%20%20
        (CallFunction|CheckPieces)
        (Audio|Components|Audio|Play (Variables|Default|Getmanhole-click-clack-41198) 0.0)))))

(event OnComponentEndOverlap(WhiteRookCol)
  (params (OverlappedComponent :type Primitive%20Component%20Object%20Reference) (OtherActor :type Actor%20Object%20Reference) (OtherComp :type Primitive%20Component%20Object%20Reference) (OtherBodyIndex :type Integer))
  (if (== OtherActor (Variables|Default|GetWhiteRook))
    (Math|Integer|DecrementInt (Variables|Default|GetPiecesOnSite))))

(event OnComponentEndOverlap(WhiteBishopCol)
  (params (OverlappedComponent :type Primitive%20Component%20Object%20Reference) (OtherActor :type Actor%20Object%20Reference) (OtherComp :type Primitive%20Component%20Object%20Reference) (OtherBodyIndex :type Integer))
  (if (== OtherActor (Variables|Default|GetWhiteBishop))
    (Math|Integer|DecrementInt (Variables|Default|GetPiecesOnSite))))

(event OnComponentBeginOverlap(BlackRookCol)
  (params (OverlappedComponent :type Primitive%20Component%20Object%20Reference) (OtherActor :type Actor%20Object%20Reference) (OtherComp :type Primitive%20Component%20Object%20Reference) (OtherBodyIndex :type Integer) (bFromSweep :type Boolean) (SweepResult :type Hit%20Result%20Structure%20%28by%20ref%29))
  (if (== OtherActor (Variables|Default|GetBlackRock))
    (Development|PrintString "Black Rook on site")
    (Math|Integer|IncrementInt (Variables|Default|GetPiecesOnSite)
      (:%20%20
        (CallFunction|CheckPieces)
        (Audio|Components|Audio|Play (Variables|Default|Getmanhole-click-clack-41196) 0.0)))))

(event OnComponentEndOverlap(BlackRookCol)
  (params (OverlappedComponent :type Primitive%20Component%20Object%20Reference) (OtherActor :type Actor%20Object%20Reference) (OtherComp :type Primitive%20Component%20Object%20Reference) (OtherBodyIndex :type Integer))
  (if (== OtherActor (Variables|Default|GetBlackRock))
    (Math|Integer|DecrementInt (Variables|Default|GetPiecesOnSite))))

(event Custom|ShowReward
  (bind _movablewall (Variables|Default|GetMovableWall))
  (AddComponent|AddAudioComponent (Variables|Default|GetMovableWall) false)
  (bind _newtrack_0 (Timeline|Timeline PlayFromStart)
    (:Update
      (Transformation|SetActorLocation _movablewall (+ (Transformation|GetActorLocation _movablewall) _newtrack_0) false false))))

(fn ConstructionScript)

(fn CheckPieces
  (if (== (Variables|Default|GetPiecesOnSite) 6)
    (Development|PrintString "All pieces in site")
    (CallFunction|ShowReward)))