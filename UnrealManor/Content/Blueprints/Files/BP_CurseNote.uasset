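; BP_CurseNote is an interactable note that toggles a text widget on screen for the player.
; Opening creates the TextWidget, clears the character's FileWidget reference, disables movement and look input, and focuses the widget in game-and-UI input mode.
; Interacting again removes the widget, forces garbage collection, and restores walking, look and game-only input.
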(event EventInteract
  (bind _returnvalue (Game|GetPlayerController 0))
  (if (Variables|Default|GetisOpen)
    (Widget|SetVisibility (Variables|Default|GetnewWidget) "Hidden")
    (Widget|RemovefromParent (Variables|Default|GetnewWidget))
    (Utilities|Platform|CollectGarbage)
    (Input|SetInputModeGameOnly (Game|GetPlayerController 0) false)
    (Variables|Default|SetisOpen false)
    (Pawn|Components|CharacterMovement|SetMovementMode (Variables|/Script/Engine.Character|GetCharacterMovement (Game|GetPlayerCharacter 0)) "MOVE_Walking" 0)
    (Input|SetIgnoreLookInput (Game|GetPlayerController 0) false)
    (else
      (Pawn|Components|CharacterMovement|DisableMovement (Variables|/Script/Engine.Character|GetCharacterMovement (Game|GetPlayerCharacter 0)))
      (bind _returnvalue_2 (UserInterface|CreateWidget (Variables|Default|GetTextWidget)))
      (bind _output_get (Variables|Default|SetnewWidget _returnvalue_2))
      (Variables|/Game/Core/FirstPerson/Blueprints/BP_FirstPersonCharacter.BP_FirstPersonCharacter_C|SetFileWidget (.AsBP%20First%20Person%20Character (Utilities|Casting|CastToBP_FirstPersonCharacter (Game|GetPlayerCharacter 0))) 0)
      (Widget|SetVisibility _output_get "Visible")
      (UserInterface|Viewport|AddtoViewport (Variables|Default|GetnewWidget) 0)
      (Input|SetIgnoreLookInput _returnvalue true)
      (Input|SetInputModeGameandUI (.AsBP%20First%20Person%20Player%20Controller (Utilities|Casting|CastToBP_FirstPersonPlayerController _returnvalue)) (Variables|Default|GetnewWidget) "DoNotLock" true false)
      (Variables|Default|SetisOpen true))))

(fn ConstructionScript)