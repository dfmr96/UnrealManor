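; BP_Final is the interactable that triggers the game's ending once the totem checker reports FinalEnabled.
; Interacting teleports the first-person character to a marker actor, hides the HUD, switches to UI-only input and plays the final audio.
; After a one-time delay it shows the credits widget, whose finished animation brings up a loading screen and opens the main menu level.
; The box overlap event is empty.
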(event OnComponentBeginOverlap(Box)
  (params (OverlappedComponent :type Primitive%20Component%20Object%20Reference) (OtherActor :type Actor%20Object%20Reference) (OtherComp :type Primitive%20Component%20Object%20Reference) (OtherBodyIndex :type Integer) (bFromSweep :type Boolean) (SweepResult :type Hit%20Result%20Structure%20%28by%20ref%29)))

(event Custom|FinishCredits
  (Widget|SetVisibility (stale EventInteract _returnvalue_2) "Hidden")
  (bind _returnvalue (UserInterface|CreateWidget "/Game/Blueprints/UI/WP_Loading.WP_Loading_C"))
  (Widget|SetVisibility _returnvalue "Visible")
  (UserInterface|Viewport|AddtoViewport _returnvalue 0)
  (Utilities|FlowControl|Delay 2.0)
  (Game|OpenLevel(byObjectReference) "/Game/LevelIglesia/MenuInicial.MenuInicial"))

(event EventInteract
  (bind _returnvalue (Game|GetPlayerCharacter 0))
  (bind _asbp_first_person_character (Utilities|Casting|CastToBP_FirstPersonCharacter _returnvalue))
  (Variables|Default|SetEnding true)
  (bind _asbp_totem_checker (Utilities|Casting|CastToBP_TotemChecker (Variables|Default|GetTotemChecker)))
  (if (Variables|/Game/Franco/Totems/BP_TotemChecker.BP_TotemChecker_C|GetFinalEnabled _asbp_totem_checker)
    (Transformation|SetActorLocation _asbp_first_person_character (Transformation|GetActorLocation (Variables|Default|GetVectorPOs)) false false)
    (Widget|SetVisibility (Variables|/Game/Core/FirstPerson/Blueprints/BP_FirstPersonCharacter.BP_FirstPersonCharacter_C|GetPlayerHUD _asbp_first_person_character) "Hidden")
    (Input|SetInputModeUIOnly (Game|GetPlayerController 0) 0 "DoNotLock" false)
    (Audio|PlaySound2D "/Game/Audio/Final_Audio.Final_Audio" 1.0 1.0 0.0 0 0)
    (Utilities|FlowControl|DoOnce false
      (:Completed
        (Utilities|FlowControl|Delay 4e+01)
        (bind _returnvalue_2 (UserInterface|CreateWidget "/Game/Blueprints/UI/WP_Credits.WP_Credits_C"))
        (Widget|SetVisibility _returnvalue_2 "Visible")
        (UserInterface|Viewport|AddtoViewport _returnvalue_2 0)
        (Class|UserWidget|BindtoAnimationFinished _returnvalue_2 (Variables|/Game/Blueprints/UI/WP_Credits.WP_Credits_C|GetCreditsAnimation _returnvalue_2) (delegate Custom|FinishCredits))))))

(fn ConstructionScript)