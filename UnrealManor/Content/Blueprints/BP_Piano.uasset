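; Piano puzzle actor that adds an audio component and moves a linked wall.
; The sequence runs on BeginPlay and again when CheckItemUsed receives an item whose row name matches ItemRequired.
; The MoveWall timeline adds its track vector to the wall's current location on each update, so movement accumulates per frame without sweeping.
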(event EventCheckItemUsed
  (params (ItemUsed :type Data%20Table%20Row%20Handle%20Structure))
  (bind _movablewall (Variables|Default|GetMovableWall))
  (if (== (.rowname ItemUsed) (.rowname (Variables|Default|GetItemRequired)))
    (AddComponent|AddAudioComponent false)
    (bind _newtrack_0 (Timeline|MoveWall PlayFromStart)
      (:Update
        (Transformation|SetActorLocation _movablewall (+ (Transformation|GetActorLocation _movablewall) _newtrack_0) false false)))))

(event EventBeginPlay
  (bind _movablewall (Variables|Default|GetMovableWall))
  (AddComponent|AddAudioComponent false)
  (bind _newtrack_0 (Timeline|MoveWall PlayFromStart)
    (:Update
      (Transformation|SetActorLocation _movablewall (+ (Transformation|GetActorLocation _movablewall) _newtrack_0) false false))))

(fn ConstructionScript)

(fn GetItemRequired
  (return ""))