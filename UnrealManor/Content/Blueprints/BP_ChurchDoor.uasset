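; BP_ChurchDoor is a two-leaf church door that opens when the metal gate opens and can be closed with sound.
; On BeginPlay it finds the BP_MetalGate actor and binds OpenChurchDoor to its GatesOpen event.
; Opening and closing each run once, snapping both leaves to fixed rotations.
; CloseChurchDoor, not called within this Blueprint, also plays audio, then a 2D voice clip after a short delay.
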(event Custom|OpenChurchDoor
  (Utilities|FlowControl|DoOnce false
    (:Completed
      (Transformation|SetRelativeRotation (Variables|Default|GetPuertaDerecha) "0.000000,270.000000,0.000000" false false)
      (Transformation|SetRelativeRotation (Variables|Default|GetPuertaIzquierda) "0.000000,-90.000000,0.000000" false false))))

(event Custom|CloseChurchDoor
  (Utilities|FlowControl|DoOnce false
    (:Completed
      (Transformation|SetRelativeRotation (Variables|Default|GetPuertaDerecha) "0.000000,180.000000,0.000000" false false)
      (Transformation|SetRelativeRotation (Variables|Default|GetPuertaIzquierda) "0, 0, 0" false false)
      (Audio|Components|Audio|Play (Variables|Default|GetAudio) 0.0)
      (Utilities|FlowControl|Delay 0.75)
      (Audio|PlaySound2D "/Game/Audio/Soundly_Voice_Designer__Tony_2.Soundly_Voice_Designer__Tony_2" 1.0 1.0 0.0 0 0))))

(event EventBeginPlay
  (bind _returnvalue (Actor|GetActorOfClass "/Game/LevelIglesia/BP_MetalGate.BP_MetalGate_C"))
  (EventDispatchers|BindEventtoGatesOpen _returnvalue (delegate Custom|OpenChurchDoor)))

(event Collision|EventActorBeginOverlap
  (params (OtherActor :type Actor%20Object%20Reference)))

(event EventTick
  (params (DeltaSeconds :type Float%20%28single-precision%29)))

(fn ConstructionScript)