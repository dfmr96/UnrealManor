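; BP_File is an interactable file in a first-person game that toggles an on-screen text widget.
; Interact creates a TextWidget, stores it on the player character's FileWidget and shows it with Game and UI input focused on it.
; Interacting again removes the widget, forces garbage collection and restores game-only input, with IsOpen tracking the state.
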(event EventInteract
  (if (Variables|Default|GetisOpen)
    (Widget|SetVisibility (Variables|Default|GetnewWidget) "Hidden")
    (Widget|RemovefromParent (Variables|Default|GetnewWidget))
    (Utilities|Platform|CollectGarbage)
    (Input|SetInputModeGameOnly (Game|GetPlayerController 0) false)
    (Variables|Default|SetisOpen false)
    (else
      (bind _returnvalue (UserInterface|CreateWidget (Variables|Default|GetTextWidget)))
      (bind _output_get (Variables|Default|SetnewWidget _returnvalue))
      (Variables|/Game/Core/FirstPerson/Blueprints/BP_FirstPersonCharacter.BP_FirstPersonCharacter_C|SetFileWidget (.AsBP%20First%20Person%20Character (Utilities|Casting|CastToBP_FirstPersonCharacter (Game|GetPlayerCharacter 0))) _returnvalue)
      (Widget|SetVisibility _output_get "Visible")
      (UserInterface|Viewport|AddtoViewport (Variables|Default|GetnewWidget) 0)
      (Input|SetInputModeGameandUI (.AsBP%20First%20Person%20Player%20Controller (Utilities|Casting|CastToBP_FirstPersonPlayerController (Game|GetPlayerController 0))) (Variables|Default|GetnewWidget) "DoNotLock" true false)
      (Variables|Default|SetisOpen true))))

(fn ConstructionScript)