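; BP_PlayerAudioForRooms is a trigger-driven audio player that starts and stops a sound as the player moves through the level.
; Overlapping Activador with player character 0 plays AudioTotem from the beginning, with the OnPlaying flag preventing restarts while it is set.
; Overlapping Pausador clears the flag and stops the audio outright, so despite its name playback does not resume where it left off.
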(event OnComponentBeginOverlap(Pausador)
  (params (OverlappedComponent :type Primitive%20Component%20Object%20Reference) (OtherActor :type Actor%20Object%20Reference) (OtherComp :type Primitive%20Component%20Object%20Reference) (OtherBodyIndex :type Integer) (bFromSweep :type Boolean) (SweepResult :type Hit%20Result%20Structure%20%28by%20ref%29))
  (if (== OtherActor (Game|GetPlayerCharacter 0))
    (Variables|Default|SetOnPlaying false)
    (Audio|Components|Audio|Stop (Variables|Default|GetAudioTotem))))

(event OnComponentBeginOverlap(Activador)
  (params (OverlappedComponent :type Primitive%20Component%20Object%20Reference) (OtherActor :type Actor%20Object%20Reference) (OtherComp :type Primitive%20Component%20Object%20Reference) (OtherBodyIndex :type Integer) (bFromSweep :type Boolean) (SweepResult :type Hit%20Result%20Structure%20%28by%20ref%29))
  (if (== OtherActor (Game|GetPlayerCharacter 0))
    (if (not (Variables|Default|GetOnPlaying))
      (Variables|Default|SetOnPlaying true)
      (Audio|Components|Audio|Play (Variables|Default|GetAudioTotem) 0.0))))

(fn ConstructionScript)