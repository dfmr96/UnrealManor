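; BP_DoorBase is an interactable door that can be locked until a required item is used on it.
; CheckItemUsed compares row names with ItemRequired to clear IsLocked.
; When unlocked, Interact drives a FlipFlop that plays or reverses a timeline rotating the mesh 90 degrees in yaw.
; An opened door loops back into the FlipFlop after a delay to auto-close, with sounds played at world origin.
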(event EventBeginPlay)

(event Collision|EventActorBeginOverlap
  (params (OtherActor :type Actor%20Object%20Reference)))

(event EventTick
  (params (DeltaSeconds :type Float%20%28single-precision%29)))

(event EventInteract
  (if (not (Variables|Default|GetisLocked?))
    (Utilities|FlowControl|FlipFlop :!label _label
      (:A
        (Variables|Default|SetisOpened? true)
        (Audio|PlaySoundatLocation "/Game/Audio/Doors__Wood__Bathroom__Open__Close_01_SND0506_1.Doors__Wood__Bathroom__Open__Close_01_SND0506_1" "0, 0, 0" "0, 0, 0" 1.0 1.0 0.0 0 0 0 0)
        (bind _doorfloat (Timeline|OpenDoor PlayFromStart)
          (:Update
            (Transformation|SetRelativeRotation (Variables|Default|GetSimpleDoorMesh) (Math|Rotator|MakeRotator 0.0 0.0 (Math|Float|Lerp 0.0 9e+01 _doorfloat)) false false))
          (:Finished
            (if (Variables|Default|GetisOpened?)
              (Utilities|FlowControl|Delay 3.0)
              (goto _label)
              (else
                (Audio|PlaySoundatLocation "/Game/Audio/Doors__Wood__Bathroom__Open__Close_01_SND0506_5.Doors__Wood__Bathroom__Open__Close_01_SND0506_5" "0, 0, 0" "0, 0, 0" 1.0 1.0 0.0 0 0 0 0))))))
      (:B
        (Variables|Default|SetisOpened? false)
        (Timeline|OpenDoor ReverseFromEnd)))))

(event EventFAddCollectable
  (params (Item_ID :type String)))

(fn ConstructionScript)

(fn CheckItemUsed
  (params (ItemUsed :type Data%20Table%20Row%20Handle%20Structure))
  (if (== (.rowname ItemUsed) (.rowname (Variables|Default|GetItemRequired)))
    (Variables|Default|SetisLocked? false)
    (return)))

(fn GetItemRequired
  (return (Variables|Default|GetItemRequired)))