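; BP_GroundItem is a world item that goes into the player's inventory when interacted with.
; Its Interact event casts player character 0 to BP_FirstPersonCharacter and asks that character's Inventory for a slot via CheckSlot.
; If the slot is empty, it loads its ItemData at that index, otherwise it only prints a message.
; The actor is not destroyed or hidden in this graph after loading.
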(event EventBeginPlay)

(event Collision|EventActorBeginOverlap
  (params (OtherActor :type Actor%20Object%20Reference)))

(event EventTick
  (params (DeltaSeconds :type Float%20%28single-precision%29)))

(event EventInteract
  (Development|PrintString "Ground item interacted")
  (bind _asbp_first_person_character (Utilities|Casting|CastToBP_FirstPersonCharacter (Game|GetPlayerCharacter 0)))
  (bind _output_get (Variables|Default|SetPlayer _asbp_first_person_character))
  (bind (_isempty _slotindex) (Default|CheckSlot (Variables|/Game/Core/FirstPerson/Blueprints/BP_FirstPersonCharacter.BP_FirstPersonCharacter_C|GetInventory _output_get)))
  (if _isempty
    (Default|LoadItem (Variables|/Game/Core/FirstPerson/Blueprints/BP_FirstPersonCharacter.BP_FirstPersonCharacter_C|GetInventory (Variables|Default|GetPlayer)) (Variables|Default|GetItemData) _slotindex)
    (Development|PrintString "Item Loaded")
    (else
      (Development|PrintString "No available slot"))))

(fn ConstructionScript)