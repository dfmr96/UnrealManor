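; Inventory item preview actor that shows the selected item's mesh on a constantly rotating model, with a SceneCaptureComponent2D alongside it.
; GetItemMesh reads the player inventory slot's row from ItemDataTable, then sets the mesh and writes name and description to the InventoryHUD.
; ResetModelView clears the mesh and fills the HUD text from the table's "null" row.
; BeginPlay removes this actor's components from the capture's show-only list.
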(event EventTick
  (params (DeltaSeconds :type Float%20%28single-precision%29))
  (Transformation|AddLocalRotation (Variables|Default|GetModelMesh) (Math|Rotator|MakeRotator 0.0 0.0 (* DeltaSeconds 2e+01)) false false))

(event EventBeginPlay
  (Class|SceneCaptureComponent|RemoveShowOnlyActorComponents (Variables|Default|GetSceneCaptureComponent2D) self false))

(fn ConstructionScript)

(fn SetModelMesh
  (params (NewParam :type Static%20Mesh%20Component%20Object%20Reference))
  (Variables|Default|SetModelMesh NewParam)
  (return))

(fn GetItemMesh
  (params (SlotId :type Integer))
  (bind _asbp_first_person_character (Utilities|Casting|CastToBP_FirstPersonCharacter (Game|GetPlayerCharacter 0)))
  (bind _returnvalue (Utilities|GetDataTableRow "/Game/Blueprints/Inventory/ItemDataTable.ItemDataTable" (.RowName (Utilities|Struct|BreakDataTableRowHandle (Utilities|Array|Get(acopy) (Variables|/Game/Blueprints/Inventory/InventoryController.InventoryController_C|GetItemData (Variables|/Game/Core/FirstPerson/Blueprints/BP_FirstPersonCharacter.BP_FirstPersonCharacter_C|GetInventory _asbp_first_person_character)) SlotId))))
    (:then
      (Components|StaticMesh|SetStaticMesh (Variables|Default|GetModelMesh) (.mesh _returnvalue))
      (bind _asbp_first_person_character_2 (Utilities|Casting|CastToBP_FirstPersonCharacter (Game|GetPlayerCharacter 0)))
      (Variables|/Script/UMG.TextBlock|SetText (Variables|/Game/Blueprints/Inventory/WBP_Inventory.WBP_Inventory_C|GetItemName (Variables|/Game/Core/FirstPerson/Blueprints/BP_FirstPersonCharacter.BP_FirstPersonCharacter_C|GetInventoryHUD _asbp_first_person_character_2)) (.name _returnvalue))
      (Variables|/Script/UMG.TextBlock|SetText (Variables|/Game/Blueprints/Inventory/WBP_Inventory.WBP_Inventory_C|GetItemDescription (Variables|/Game/Core/FirstPerson/Blueprints/BP_FirstPersonCharacter.BP_FirstPersonCharacter_C|GetInventoryHUD _asbp_first_person_character_2)) (.description _returnvalue)))))

(fn ResetModelView
  (bind _returnvalue (Utilities|GetDataTableRow "/Game/Blueprints/Inventory/ItemDataTable.ItemDataTable" "null")
    (:then
      (Components|StaticMesh|SetStaticMesh (Variables|Default|GetModelMesh) 0)
      (bind _asbp_first_person_character (Utilities|Casting|CastToBP_FirstPersonCharacter (Game|GetPlayerCharacter 0)))
      (Variables|/Script/UMG.TextBlock|SetText (Variables|/Game/Blueprints/Inventory/WBP_Inventory.WBP_Inventory_C|GetItemName (Variables|/Game/Core/FirstPerson/Blueprints/BP_FirstPersonCharacter.BP_FirstPersonCharacter_C|GetInventoryHUD _asbp_first_person_character)) (.name _returnvalue))
      (Variables|/Script/UMG.TextBlock|SetText (Variables|/Game/Blueprints/Inventory/WBP_Inventory.WBP_Inventory_C|GetItemDescription (Variables|/Game/Core/FirstPerson/Blueprints/BP_FirstPersonCharacter.BP_FirstPersonCharacter_C|GetInventoryHUD _asbp_first_person_character)) (.description _returnvalue)))))