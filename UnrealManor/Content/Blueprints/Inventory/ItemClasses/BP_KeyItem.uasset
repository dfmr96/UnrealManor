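; BP_KeyItem is a usable key inventory item that is checked against whatever object currently requires an item from the player.
; Its construction script fills ItemData with a hardcoded test name, image and self/class references, and sets the body mesh.
; UseItem reads the player character's ItemRequirer through BPI_ItemRequirer and compares the required row name to the item's name.
; On a match it passes its data table row to CheckItemUsed, with debug prints throughout.
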(event EventBeginPlay
  (|CallParentFunction) ; This node is disabled and will not be called.\nDrag off pins to build functionality.
)

(event Collision|EventActorBeginOverlap
  (params (OtherActor :type Actor%20Object%20Reference))
  (|CallParentFunction OtherActor) ; This node is disabled and will not be called.\nDrag off pins to build functionality.
)

(event EventTick
  (params (DeltaSeconds :type Float%20%28single-precision%29))
  (|CallParentFunction DeltaSeconds) ; This node is disabled and will not be called.\nDrag off pins to build functionality.
)

(event EventUseItem
  (Development|PrintString "Key used 1")
  (bind _asbp_first_person_character (Utilities|Casting|CastToBP_FirstPersonCharacter (Game|GetPlayerCharacter 0)))
  (Development|PrintString "player casted")
  (bind _asbpi_item_requirer (Utilities|Casting|CastToBPI_ItemRequirer (Variables|/Game/Core/FirstPerson/Blueprints/BP_FirstPersonCharacter.BP_FirstPersonCharacter_C|GetItemRequirer _asbp_first_person_character)))
  (bind _itemrequired (Default|GetItemRequired _asbpi_item_requirer))
  (Development|PrintString "samei tem" (== (Utilities|String|StringToName (Utilities|String|ToString(Text) (.name (Variables|Default|GetItemData)))) (.rowname _itemrequired)))
  (if (== (Utilities|String|StringToName (Utilities|String|ToString(Text) (.name (Variables|Default|GetItemData)))) (.rowname _itemrequired))
    (Default|CheckItemUsed _asbpi_item_requirer (Variables|Default|GetItemDataTableRow))
    (else
      (Development|PrintString "are same item"))))

(fn ConstructionScript
  (Variables|Default|SetItemData (Utilities|Struct|MakeItemData "TestKey" "" "" "" (Variables|Default|GetImage2D) self "BP_KeyItem_C"))
  (Components|StaticMesh|SetStaticMesh (Variables|Default|GetBody) (Variables|Default|GetObject3D)))