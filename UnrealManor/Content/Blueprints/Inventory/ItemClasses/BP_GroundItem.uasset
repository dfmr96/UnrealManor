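; Base or generic pickup actor for an item lying in the world, which the player collects into their inventory.
; InitData, run from the construction script, looks up the item's data table row to set the mesh and amount, using the row's default when zero is passed.
; Interact loads the item data into a free slot of the first-person character's inventory, but never removes the actor.
; UseItem is a stub returning false.
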(event EventInteract
  (Development|PrintString "Ground item interacted")
  (bind _asbp_first_person_character (Utilities|Casting|CastToBP_FirstPersonCharacter (Game|GetPlayerCharacter 0)))
  (bind _output_get (Variables|Default|SetPlayer _asbp_first_person_character))
  (bind (_isempty _slotindex) (Default|CheckSlot (Variables|/Game/Core/FirstPerson/Blueprints/BP_FirstPersonCharacter.BP_FirstPersonCharacter_C|GetInventory _output_get)))
  (if _isempty
    (Default|LoadItem (Variables|/Game/Core/FirstPerson/Blueprints/BP_FirstPersonCharacter.BP_FirstPersonCharacter_C|GetInventory (Variables|Default|GetPlayer)) (Variables|Default|GetItemData) _slotindex)
    (Development|PrintString "Item Loaded")
    (else
      (Development|PrintString "No available slot"))))

(fn ConstructionScript
  (CallFunction|InitData))

(fn UseItem
  (return false))

(fn InitData
  (params (NewAmount :type Integer))
  (bind _returnvalue (Utilities|GetDataTableRow "/Game/Blueprints/Inventory/ItemDataTable.ItemDataTable" (.rowname (Variables|Default|GetItemData)))
    (:then
      (Components|StaticMesh|SetStaticMesh (Variables|Default|GetBody) (.mesh _returnvalue))
      (if (== NewAmount 0)
        (Variables|Default|SetAmount (.amount _returnvalue))
        (else
          (Variables|Default|SetAmount NewAmount))))))