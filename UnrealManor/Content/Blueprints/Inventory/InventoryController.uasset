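; Inventory controller that stores the player's items in a slot array and registers itself with the first-person character on BeginPlay.
; CheckSlot finds the first free slot, treating a missing image as empty, and LoadItem fills a slot and destroys the character's ground item.
; UnloadItem clears a slot and respawns the item at the character's mesh.
; RenderInventory updates HUD slot icons, frames and visibility, bounded by CurrentSize.
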(event EventBeginPlay
  (bind _asbp_first_person_character (Utilities|Casting|CastToBP_FirstPersonCharacter (Game|GetPlayerCharacter 0)))
  (Variables|/Game/Core/FirstPerson/Blueprints/BP_FirstPersonCharacter.BP_FirstPersonCharacter_C|SetInventory _asbp_first_person_character self))

(fn ConstructionScript)

(fn CheckSlot
  (LocalVariables|SetEmptySlot -2)
  (bind (_array_element _array_index) (Utilities|Array|ForEachLoopwithBreak (Variables|Default|GetItemData) :!label _label)
    (:LoopBody
      (if (== (.image _array_element) 0)
        (LocalVariables|SetEmptySlot _array_index)
        (goto _label Break)))
    (:Completed
      (if (== (LocalVariables|GetEmptySlot) -2)
        (return false (LocalVariables|GetEmptySlot))
        (else
          (return true (LocalVariables|GetEmptySlot)))))))

(fn LoadItem
  (params (ItemData :type Item%20Data%20Structure) (SlotIndex :type Integer))
  (LocalVariables|SetItemToAdd ItemData)
  (bind _output_get (LocalVariables|SetSlot SlotIndex))
  (if (Math|Integer|InRange(Integer) _output_get 0 (Variables|Default|GetCurrentSize))
    (Utilities|Array|SetArrayElem (Variables|Default|GetItemData) (LocalVariables|GetSlot) (LocalVariables|GetItemToAdd))
    (Actor|DestroyActor (Variables|/Game/Core/FirstPerson/Blueprints/BP_FirstPersonCharacter.BP_FirstPersonCharacter_C|GetGroundItem (.AsBP%20First%20Person%20Character (Utilities|Casting|CastToBP_FirstPersonCharacter (Game|GetPlayerCharacter 0)))))))

(fn UnloadItem
  (params (ItemData :type Item%20Data%20Structure) (SlotIndex :type Integer))
  (LocalVariables|SetLoadedItem ItemData)
  (Utilities|Array|SetArrayElem :TargetArray (Variables|Default|GetItemData) :Index SlotIndex)
  (bind _returnvalue (Game|SpawnActorfromClass (.objectclass (LocalVariables|GetLoadedItem)) (Transformation|GetWorldTransform (Variables|/Script/Engine.Character|GetMesh (.AsBP%20First%20Person%20Character (Utilities|Casting|CastToBP_FirstPersonCharacter (Game|GetPlayerCharacter 0))))) "Undefined" "MultiplyWithRoot" 0 0))
  (bind _asbp_ground_item (Utilities|Casting|CastToBP_GroundItem _returnvalue))
  (Variables|/Game/Blueprints/Inventory/ItemClasses/BP_GroundItem.BP_GroundItem_C|SetItemData _asbp_ground_item (Utilities|Struct|MakeItemData (.name (LocalVariables|GetLoadedItem)) (.type (LocalVariables|GetLoadedItem)) (.description (LocalVariables|GetLoadedItem)) "" (.image (LocalVariables|GetLoadedItem)) _asbp_ground_item (.objectclass (LocalVariables|GetLoadedItem)))))

(fn RenderInventory
  (bind (_array_element _array_index) (Utilities|Array|ForEachLoopwithBreak (Variables|Default|GetItemData) :!label _label)
    (:LoopBody
      (LocalVariables|SetcurrentItem _array_element)
      (LocalVariables|SetcurrentSlotIndex _array_index)
      (if (<= _array_index (Variables|Default|GetCurrentSize))
        (bind _aswbp_inventory_slot (Utilities|Casting|CastToWBP_InventorySlot (Class|PanelWidget|GetChildat (Variables|/Game/Blueprints/Inventory/WBP_Inventory.WBP_Inventory_C|GetInventoryPanel (Variables|/Game/Core/FirstPerson/Blueprints/BP_FirstPersonCharacter.BP_FirstPersonCharacter_C|GetInventoryHUD (.AsBP%20First%20Person%20Character (Utilities|Casting|CastToBP_FirstPersonCharacter (Game|GetPlayerCharacter 0))))) (LocalVariables|GetcurrentSlotIndex))))
        (bind _output_get (LocalVariables|SetcurrentSlot _aswbp_inventory_slot))
        (Variables|/Script/UMG.Widget|SetVisibility _output_get "Visible")
        (Appearance|SetBrushfromTexture (Variables|/Game/Blueprints/Inventory/WBP_InventorySlot.WBP_InventorySlot_C|GetItem (LocalVariables|GetcurrentSlot)) (.image (LocalVariables|GetcurrentItem)))
        (if (== (.image (LocalVariables|GetcurrentItem)) 0)
          (Class|Border|SetBrush (Variables|/Game/Blueprints/Inventory/WBP_InventorySlot.WBP_InventorySlot_C|GetFrame (LocalVariables|GetcurrentSlot)) (Class|PaperSpriteBlueprintLibrary|MakeBrushfromSprite "/Game/Blueprints/Inventory/Sprites/T_UI_Sprite_0.T_UI_Sprite_0"))
          (Variables|/Script/UMG.Widget|SetVisibility (Variables|/Game/Blueprints/Inventory/WBP_InventorySlot.WBP_InventorySlot_C|GetItem (LocalVariables|GetcurrentSlot)) "Hidden")
          (else
            (Class|Border|SetBrush (Variables|/Game/Blueprints/Inventory/WBP_InventorySlot.WBP_InventorySlot_C|GetFrame (LocalVariables|GetcurrentSlot)) (Class|PaperSpriteBlueprintLibrary|MakeBrushfromSprite "/Game/Blueprints/Inventory/Sprites/T_UI_Sprite_1.T_UI_Sprite_1"))
            (Variables|/Script/UMG.Widget|SetVisibility (Variables|/Game/Blueprints/Inventory/WBP_InventorySlot.WBP_InventorySlot_C|GetItem (LocalVariables|GetcurrentSlot)) "Visible")))
        (else
          (goto _label Break))))))