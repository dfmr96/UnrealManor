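; Double door actor built from two BP_DoorBase child actors, which unlock together when the player reaches it.
; The first player overlap of its Box trigger passes a DoOnce, unlocks both doors and plays a key-jingle sound.
; No item is checked for unlocking: CheckItemUsed only clears the player's text prompt or says the item can't be used here, and GetItemRequired is empty.
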(event OnComponentBeginOverlap(Box)
  (params (OverlappedComponent :type Primitive%20Component%20Object%20Reference) (OtherActor :type Actor%20Object%20Reference) (OtherComp :type Primitive%20Component%20Object%20Reference) (OtherBodyIndex :type Integer) (bFromSweep :type Boolean) (SweepResult :type Hit%20Result%20Structure%20%28by%20ref%29))
  (if (== OtherActor (Game|GetPlayerCharacter 0))
    (Utilities|FlowControl|DoOnce false
      (:Completed
        (Default|UnlockDoor (.AsBP%20Door%20Base (Utilities|Casting|CastToBP_DoorBase (Variables|/Script/Engine.ChildActorComponent|GetChildActor (Variables|Default|GetBP_DoorBase1)))))
        (Default|UnlockDoor (.AsBP%20Door%20Base (Utilities|Casting|CastToBP_DoorBase (Variables|/Script/Engine.ChildActorComponent|GetChildActor (Variables|Default|GetBP_DoorBase2)))))
        (Audio|PlaySound2D "/Game/Audio/Doors__Hardware__Wood__Unlocking__Key_Jingle__Slight_Room_Reverb_SND26176_1.Doors__Hardware__Wood__Unlocking__Key_Jingle__Slight_Room_Reverb_SND26176_1" 1.0 1.0 0.0 0 0)))))

(fn ConstructionScript)

(fn CheckItemUsed
  (params (ItemUsed :type Data%20Table%20Row%20Handle%20Structure))
  (bind _returnvalue (Game|GetPlayerCharacter 0))
  (bind _asbp_first_person_character (Utilities|Casting|CastToBP_FirstPersonCharacter _returnvalue))
  (bind _textprompter (Variables|/Game/Core/FirstPerson/Blueprints/BP_FirstPersonCharacter.BP_FirstPersonCharacter_C|GetTextPrompter _asbp_first_person_character))
  (if (== (.rowname ItemUsed) "")
    (Default|WriteText _textprompter)
    (else
      (Default|WriteText _textprompter "Cant use this item here"))))

(fn GetItemRequired
  (return ""))