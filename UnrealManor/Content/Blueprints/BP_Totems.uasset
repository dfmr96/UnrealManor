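; BP_Totems is an interactable puzzle totem that the player burns using a required item.
; Interacting shows its unburnt text through the first-person character's TextPrompter.
; CheckItemUsed compares item row names; a match shows burning text, marks it burnt, restores PFire's time dilation and calls TotemChecker's CheckFinal, while a mismatch shows a hint.
; A near-duplicate event, CheckItemUsed_1_1, omits the CheckFinal call.
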(event Custom|CheckItemUsed_1_1
  (params (ItemUsed :type Data%20Table%20Row%20Handle%20Structure) (ItemUsed_DataTable :type Data%20Table%20Object%20Reference) (ItemUsed_RowName :type Name))
  (bind _returnvalue (Game|GetPlayerCharacter 0))
  (bind _asbp_first_person_character (Utilities|Casting|CastToBP_FirstPersonCharacter _returnvalue))
  (bind _textprompter (Variables|/Game/Core/FirstPerson/Blueprints/BP_FirstPersonCharacter.BP_FirstPersonCharacter_C|GetTextPrompter _asbp_first_person_character))
  (if (== (.rowname ItemUsed) (.rowname (Variables|Default|GetItemRequired_1)))
    (Default|WriteText _textprompter (Variables|Default|GetBurningText))
    (Variables|Default|SetisBurnt? true)
    (Variables|/Script/Engine.ParticleSystemComponent|SetCustomTimeDilation (Variables|Default|GetP_Fire) 1.0)
    (else
      (Default|WriteText _textprompter "I just need something to Burn"))))

(event EventInteract
  (Default|WriteText (Variables|/Game/Core/FirstPerson/Blueprints/BP_FirstPersonCharacter.BP_FirstPersonCharacter_C|GetTextPrompter (.AsBP%20First%20Person%20Character (Utilities|Casting|CastToBP_FirstPersonCharacter (Game|GetPlayerCharacter 0)))) (Variables|Default|GetUnBurntText)))

(fn ConstructionScript)

(fn CheckItemUsed
  (params (ItemUsed :type Data%20Table%20Row%20Handle%20Structure))
  (bind _returnvalue (Game|GetPlayerCharacter 0))
  (bind _asbp_first_person_character (Utilities|Casting|CastToBP_FirstPersonCharacter _returnvalue))
  (bind _textprompter (Variables|/Game/Core/FirstPerson/Blueprints/BP_FirstPersonCharacter.BP_FirstPersonCharacter_C|GetTextPrompter _asbp_first_person_character))
  (if (== (.rowname ItemUsed) (.rowname (Variables|Default|GetItemRequired_1)))
    (Default|WriteText _textprompter (Variables|Default|GetBurningText))
    (Variables|Default|SetisBurnt? true)
    (Variables|/Script/Engine.ParticleSystemComponent|SetCustomTimeDilation (Variables|Default|GetP_Fire) 1.0)
    (Default|CheckFinal (Variables|Default|GetTotemChecker))
    (return true)
    (else
      (Default|WriteText _textprompter "I just need something to burn")
      (return false))))

(fn GetItemRequired
  (return ""))