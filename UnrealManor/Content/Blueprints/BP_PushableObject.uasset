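; Block actor that the player can push along cardinal axes or climb onto, with separate overlap colliders enabling each action.
; A player Hit snaps their forward vector to an axis, then CanPush line-traces the block and box-traces the destination for obstacles.
; A valid push attaches the movement-disabled player while the MoveBlock timeline slides the block by PushDistance, then releases them.
; Interact runs another timeline that lerps the player toward a bounds-derived point above the block.
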(event OnComponentBeginOverlap(InteractCollider)
  (params (OverlappedComponent :type Primitive%20Component%20Object%20Reference) (OtherActor :type Actor%20Object%20Reference) (OtherComp :type Primitive%20Component%20Object%20Reference) (OtherBodyIndex :type Integer) (bFromSweep :type Boolean) (SweepResult :type Hit%20Result%20Structure%20%28by%20ref%29))
  ;[1 1 1] Chequeo colisionador para interactuar
  (if (== OtherActor (Game|GetPlayerCharacter 0))
    (Variables|Default|SetCanClimb true)
    (Development|PrintString "Press E to Interact" false)))

(event OnComponentBeginOverlap(PushCollider)
  (params (OverlappedComponent :type Primitive%20Component%20Object%20Reference) (OtherActor :type Actor%20Object%20Reference) (OtherComp :type Primitive%20Component%20Object%20Reference) (OtherBodyIndex :type Integer) (bFromSweep :type Boolean) (SweepResult :type Hit%20Result%20Structure%20%28by%20ref%29))
  ;[1 1 1] Chequeo colisionador para empujar
  (if (== OtherActor (Game|GetPlayerCharacter 0))
    (Variables|Default|SetReadyToPush true)))

(event OnComponentEndOverlap(PushCollider)
  (params (OverlappedComponent :type Primitive%20Component%20Object%20Reference) (OtherActor :type Actor%20Object%20Reference) (OtherComp :type Primitive%20Component%20Object%20Reference) (OtherBodyIndex :type Integer))
  ;[1 1 1] Chequeo colisionador para empujar
  (if (== (Game|GetPlayerCharacter 0) OtherActor)
    (Variables|Default|SetReadyToPush false)
    (Variables|Default|SetAlreadyPushing false)))

(event OnComponentEndOverlap(InteractCollider)
  (params (OverlappedComponent :type Primitive%20Component%20Object%20Reference) (OtherActor :type Actor%20Object%20Reference) (OtherComp :type Primitive%20Component%20Object%20Reference) (OtherBodyIndex :type Integer))
  ;[1 1 1] Chequeo colisionador para interactuar
  (if (== (Game|GetPlayerCharacter 0) OtherActor)
    (Variables|Default|SetCanClimb false)
    (Development|PrintString "out of range" false)))

(event Custom|Push
  ;[1 1 1] Empujar y parar de empujar
  (Variables|Default|SetCurrentLocation (Transformation|GetActorLocation))
  (if (Variables|Default|GetAlreadyPushing)
    (bind _position (Timeline|MoveBlock Play)
      (:Update
        (Variables|Default|SetAlreadyPushing true)
        (Transformation|SetActorRelativeLocation (+ (Variables|Default|GetCurrentLocation) (* _position (Variables|Default|GetPushableDirection) (Variables|Default|GetPushDistance)))))
      (:Finished
        (CallFunction|StopPushing)))
    (else
      (Timeline|MoveBlock PlayFromStart))))

(event Custom|StopPushing
  (bind _returnvalue (Game|GetPlayerCharacter 0))
  ;[1 1 1] Empujar y parar de empujar
  (Pawn|Components|CharacterMovement|SetMovementMode (Variables|/Script/Engine.Character|GetCharacterMovement _returnvalue) "MOVE_Walking" 0)
  (Transformation|DetachFromActor _returnvalue "KeepWorld" "KeepWorld" "KeepWorld"))

(event EventInteract
  (bind _returnvalue (Game|GetPlayerCharacter 0))
  (bind _self self)
  ;[1 1 1] Climb
  (if (Variables|Default|GetCanClimb)
    (bind _center (Collision|GetActorArrayBounds (Utilities|Array|MakeArray _self)))
    (bind _newtrack_0 (Timeline|Timeline PlayFromStart)
      (:Update
        (Transformation|SetActorLocation _returnvalue (Math|Vector|Lerp(Vector) (Transformation|GetActorLocation _returnvalue) (+ (Transformation|GetActorLocation _self) (Math|Vector|MakeVector 0.0 0.0 (/ (+ (Math|Float|Power (.x (- _center (Transformation|GetActorLocation _self))) 2.0) (Math|Float|Power (.y (- _center (Transformation|GetActorLocation _self))) 2.0) (Math|Float|Power (.z (- _center (Transformation|GetActorLocation _self))) 2.0)) 2e+01))) _newtrack_0) false true)))))

(event Collision|EventHit
  (params (MyComp :type Primitive%20Component%20Object%20Reference) (Other :type Actor%20Object%20Reference) (OtherComp :type Primitive%20Component%20Object%20Reference) (bSelfMoved :type Boolean) (HitLocation :type Vector :default "0, 0, 0") (HitNormal :type Vector :default "0, 0, 0") (NormalImpulse :type Vector :default "0, 0, 0") (Hit :type Hit%20Result%20Structure%20%28by%20ref%29))
  (bind _returnvalue (Transformation|GetActorForwardVector Other))
  (bind _returnvalue_2 (Game|GetPlayerCharacter 0))
  (bind (_x _y _z) (Math|Vector|BreakVector _returnvalue))
  (bind _returnvalue_3 (Math|Float|Round _x))
  (bind _returnvalue_4 (Math|Float|Round _y))
  (if (Variables|Default|GetReadyToPush)
    (if (== Other (Game|GetPlayerCharacter 0))
      (Variables|Default|SetPushableDirection (Math|Vector|MakeVector (* (Math|Conversions|ToFloat(Integer) _returnvalue_3) (Math|Conversions|ToFloat(Boolean) (not (!= _returnvalue_4 0)))) (* (Math|Conversions|ToFloat(Integer) _returnvalue_4) (Math|Conversions|ToFloat(Boolean) (not (!= _returnvalue_3 0)))) (Math|Conversions|ToFloat(Integer) (Math|Float|Round _z))))
      (bind _canpush (CallFunction|CanPush))
      (if _canpush
        (Pawn|Components|CharacterMovement|DisableMovement (Variables|/Script/Engine.Character|GetCharacterMovement _returnvalue_2))
        (Transformation|AttachActorToActor _returnvalue_2 self "None" "KeepWorld" "KeepWorld" "KeepWorld" true)
        (CallFunction|Push)))))

(fn ConstructionScript)

(fn CanPush
  (bind _returnvalue (Game|GetPlayerCharacter 0))
  (bind _returnvalue_2 (Transformation|GetActorLocation))
  (bind _returnvalue_3 (Transformation|GetActorLocation _returnvalue))
  (bind (_outhit _returnvalue_4) (Collision|LineTraceByChannel _returnvalue_3 (+ _returnvalue_3 (* (Transformation|GetActorForwardVector _returnvalue) 1e+02)) "TraceTypeQuery1" false (Utilities|Array|MakeArray _returnvalue) "None" false))
  (if _returnvalue_4
    (if (== (.HitActor (Collision|BreakHitResult _outhit)) self)
      ;[1 1 1] Dibuja una el mesh del actor para chequear distancia con otros objetos y bloquear movimiento.
      (bind _returnvalue_5 (Collision|BoxTraceByChannel (+ _returnvalue_2 (Math|Vector|MakeVector 0.0 0.0 1e+02)) (+ _returnvalue_2 (* (Variables|Default|GetPushableDirection) (Variables|Default|GetPushDistance)) (Math|Vector|MakeVector 0.0 0.0 1e+02)) (* (.boxextent (StaticMesh|GetBounds (Variables|/Script/Engine.StaticMeshComponent|GetStaticMesh (Variables|Default|GetCube)))) (Variables|/Script/Engine.SceneComponent|GetRelativeScale3D (Variables|Default|GetCube))) "0, 0, 0" "TraceTypeQuery1" false 0 "None"))
      (return (not _returnvalue_5))
      (else
        (return false)))
    (else
      (return false))))