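; BP_ChurchWall is a church wall actor with a two-part door that slides open when triggered through the altar.
; On BeginPlay it finds the BP_Altar actor and hands it the Open_ChurchDoor event through AssignInteraction.
; That event sets DoorState so it runs only once, then slides Izquierda and Derecha in opposite directions with a looping Delay until Izquierda reaches its Y limit.
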(event Custom|Open_ChurchDoor
  (bind _izquierda (Variables|Default|GetIzquierda))
  (if (not (Variables|Default|GetDoor_State))
    (Variables|Default|SetDoor_State true)
    (if (< (.y (Variables|/Script/Engine.SceneComponent|GetRelativeLocation _izquierda)) 225.0) :!label _label
      (Transformation|AddLocalOffset _izquierda (Math|Vector|MakeVector 0.0 1.0 0.0) false false)
      (Transformation|AddLocalOffset (Variables|Default|GetDerecha) (Math|Vector|MakeVector 0.0 -1.0 0.0) false false)
      (Utilities|FlowControl|Delay 0.01)
      (goto _label))))

(event EventBeginPlay
  (bind _returnvalue (Actor|GetActorOfClass "/Game/Blueprints/BP_Altar.BP_Altar_C"))
  (EventDispatchers|AssignInteraction _returnvalue (delegate Custom|Open_ChurchDoor)))

(event Collision|EventActorBeginOverlap
  (params (OtherActor :type Actor%20Object%20Reference)))

(event EventTick
  (params (DeltaSeconds :type Float%20%28single-precision%29)))

(fn ConstructionScript)