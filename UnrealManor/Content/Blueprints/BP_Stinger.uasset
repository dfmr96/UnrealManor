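; BP_Stinger is a one-shot, two-stage encounter trigger that spawns an enemy and arms the player.
; When the player enters DetectionZone, it sets PlayerPass, spawns a BP_Romero at the Arrow, applies its configured health and damage, and calls StandUp.
; When the player enters TriggerZone with PlayerPass set, it plays the audio and enables the player's gun.
; DoOnce nodes keep each stage from repeating.
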(event OnComponentBeginOverlap(DetectionZone)
  (params (OverlappedComponent :type Primitive%20Component%20Object%20Reference) (OtherActor :type Actor%20Object%20Reference) (OtherComp :type Primitive%20Component%20Object%20Reference) (OtherBodyIndex :type Integer) (bFromSweep :type Boolean) (SweepResult :type Hit%20Result%20Structure%20%28by%20ref%29))
  (bind _arrow (Variables|Default|GetArrow))
  (if (== OtherActor (.AsBP%20First%20Person%20Character (Utilities|Casting|CastToBP_FirstPersonCharacter (Game|GetPlayerCharacter 0))))
    (Variables|Default|SetPlayerPass true)
    (Utilities|FlowControl|DoOnce false
      (:Completed
        (bind _returnvalue (Game|SpawnActorfromClass "/Game/Franco/Romero/BP_Romero.BP_Romero_C" (Math|Transform|MakeTransform (Transformation|GetWorldLocation _arrow) (Transformation|GetWorldRotation _arrow) "1.000000,1.000000,1.000000") "AdjustIfPossibleButAlwaysSpawn" "MultiplyWithRoot" 0 0))
        (Variables|/Game/Franco/Romero/BP_Romero.BP_Romero_C|SetHealth _returnvalue (Variables|Default|GetEnemyHealth))
        (Variables|/Game/Franco/Romero/BP_Romero.BP_Romero_C|SetDamage _returnvalue (Variables|Default|GetEnemyDamage))
        (Default|StandUp _returnvalue)))))

(event OnComponentBeginOverlap(TriggerZone)
  (params (OverlappedComponent :type Primitive%20Component%20Object%20Reference) (OtherActor :type Actor%20Object%20Reference) (OtherComp :type Primitive%20Component%20Object%20Reference) (OtherBodyIndex :type Integer) (bFromSweep :type Boolean) (SweepResult :type Hit%20Result%20Structure%20%28by%20ref%29))
  (bind _returnvalue (Game|GetPlayerCharacter 0))
  (bind _asbp_first_person_character (Utilities|Casting|CastToBP_FirstPersonCharacter _returnvalue))
  (if (== OtherActor _asbp_first_person_character)
    (if (Variables|Default|GetPlayerPass)
      (Utilities|FlowControl|DoOnce false
        (:Completed
          (Audio|Components|Audio|Play (Variables|Default|GetAudio) 0.0)
          (Default|EnableGun _asbp_first_person_character))))))

(fn ConstructionScript)