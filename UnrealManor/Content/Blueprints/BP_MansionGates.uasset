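; BP_MansionGates is the mansion gate Blueprint, which shuts its two gates with audio cues when the CloseMansionGates event is called.
; A DoOnce limits the event to a single run, snapping both gate components to zero relative rotation without animation and printing debug messages.
; It then plays a 2D thunder sound, followed by church bells after a short delay.
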(event Custom|CloseMansionGates
  (Utilities|FlowControl|DoOnce false
    (:Completed
      (Development|PrintString "OnMansionGate")
      (Variables|Default|SetGate_RightGate (Variables|Default|GetGate_RightGate))
      (Development|PrintString "Right Gate Closed")
      (Transformation|SetRelativeRotation (Variables|Default|GetGate_RightGate) "0, 0, 0" false false)
      (Development|PrintString "Left Gate Closed")
      (Variables|Default|SetGate_LeftGate (Variables|Default|GetGate_LeftGate))
      (Transformation|SetRelativeRotation (Variables|Default|GetGate_LeftGate) "0, 0, 0" false false)
      (Audio|PlaySound2D "/Game/Audio/mixkit-distant-thunder-explosion-1278.mixkit-distant-thunder-explosion-1278" 1.0 1.0 0.0 0 0)
      (Utilities|FlowControl|Delay 3.0)
      (Audio|PlaySound2D "/Game/Audio/oldchurchbell_x3.oldchurchbell_x3" 1.0 1.0 0.0 0 0))))

(fn ConstructionScript)