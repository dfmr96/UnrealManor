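; BP_Cube is a pushable cube that moves with the first-person character's input while the player interacts with it.
; Overlapping its PusheableTrigger sets CanInteractBox on the cached BP_FirstPersonCharacter, without checking the overlapping actor.
; Each Tick, while both interaction flags are true, the character's axis values choose the direction and sign passed to MoveDirection.
; MoveDirection offsets the mesh's relative location along its right or forward vector using VInterpTo, without sweep.
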(event OnComponentBeginOverlap(PusheableTrigger)
  (params (OverlappedComponent :type Primitive%20Component%20Object%20Reference) (OtherActor :type Actor%20Object%20Reference) (OtherComp :type Primitive%20Component%20Object%20Reference) (OtherBodyIndex :type Integer) (bFromSweep :type Boolean) (SweepResult :type Hit%20Result%20Structure%20%28by%20ref%29))
  (Development|PrintString "Character can move cube")
  (Variables|/Game/FirstPerson/Blueprints/BP_FirstPersonCharacter.BP_FirstPersonCharacter_C|SetCanInteractBox? (Variables|Default|GetCharacter%20Reference) true))

(event OnComponentEndOverlap(PusheableTrigger)
  (params (OverlappedComponent :type Primitive%20Component%20Object%20Reference) (OtherActor :type Actor%20Object%20Reference) (OtherComp :type Primitive%20Component%20Object%20Reference) (OtherBodyIndex :type Integer))
  (Development|PrintString "Character outside pusheable bounds")
  (Variables|/Game/FirstPerson/Blueprints/BP_FirstPersonCharacter.BP_FirstPersonCharacter_C|SetCanInteractBox? (Variables|Default|GetCharacter%20Reference) false))

(event EventBeginPlay
  (bind _returnvalue (Actor|GetActorOfClass "/Game/FirstPerson/Blueprints/BP_FirstPersonCharacter.BP_FirstPersonCharacter_C"))
  (Variables|Default|SetCharacter%20Reference _returnvalue))

(event Collision|EventActorBeginOverlap
  (params (OtherActor :type Actor%20Object%20Reference)))

(event EventTick
  (params (DeltaSeconds :type Float%20%28single-precision%29))
  (bind _character_reference (Variables|Default|GetCharacter%20Reference))
  (bind _character_reference_2 (Variables|Default|GetCharacter%20Reference))
  (bind _vertical_axis (Variables|/Game/FirstPerson/Blueprints/BP_FirstPersonCharacter.BP_FirstPersonCharacter_C|GetVertical%20Axis _character_reference_2))
  (bind _horizontal_axis (Variables|/Game/FirstPerson/Blueprints/BP_FirstPersonCharacter.BP_FirstPersonCharacter_C|GetHorizontal%20Axis _character_reference_2))
  (if (Variables|/Game/FirstPerson/Blueprints/BP_FirstPersonCharacter.BP_FirstPersonCharacter_C|GetIsInteractingBox? _character_reference)
    (if (Variables|/Game/FirstPerson/Blueprints/BP_FirstPersonCharacter.BP_FirstPersonCharacter_C|GetCanInteractBox? _character_reference)
      (Utilities|FlowControl|Sequence
        (:then_0
          (if (== _vertical_axis 0.0)
            (Development|PrintString "Player not moving on Y axis")
            (elif (>= _vertical_axis 0.5)
              (Development|PrintString "Player moving forward")
              (Utilities|Move/Direction true -25.0)
              (else
                (Development|PrintString "Player moving backwards")
                (Utilities|Move/Direction true 25.0)))))
        (:then_1
          (if (== _horizontal_axis 0.0)
            (Development|PrintString "Player not moving on Y axis")
            (elif (>= _horizontal_axis 0.5)
              (Development|PrintString "Player moving left")
              (Utilities|Move/Direction false 25.0)
              (else
                (Development|PrintString "Player moving right")
                (Utilities|Move/Direction false -25.0)))))))))

(fn ConstructionScript)