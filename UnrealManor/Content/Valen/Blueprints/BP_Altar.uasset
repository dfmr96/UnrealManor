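; Altar that takes required items from the player's inventory and reveals the matching cross and Jesus meshes as they are placed.
; On interaction, it loops over the first-person character's Inventario against RequireItems, removing matches from both arrays during iteration.
; Each match passes its item ID to a custom event that shows the corresponding component.
; CallInteraction fires inside the outer loop whenever RequireItems is empty, so it can repeat.
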(event Custom|CE_ActiveChurchObjects
  (params (ObjectToActivate :type String))
  (if (Utilities|Enum|Equal(Enum) ObjectToActivate "Item01")
    (Rendering|SetVisibility (Variables|Default|GetCruz_Entera_Cruz_1) true false)
    (elif (Utilities|Enum|Equal(Enum) ObjectToActivate "Item02")
      (Rendering|SetVisibility (Variables|Default|GetCruz_Entera_Cruz_2) true false)
      (elif (Utilities|Enum|Equal(Enum) ObjectToActivate "Item03")
        (Rendering|SetVisibility (Variables|Default|GetCruz_Entera_Jesus) true false)))))

(event EventBeginPlay)

(event EventFInteraction
  (bind _returnvalue (Actor|GetActorOfClass "/Game/FirstPerson/Blueprints/BP_FirstPersonCharacter.BP_FirstPersonCharacter_C"))
  (for _array_element (Variables|/Game/FirstPerson/Blueprints/BP_FirstPersonCharacter.BP_FirstPersonCharacter_C|GetInventario _returnvalue)
    (for _array_element_2 (Variables|Default|GetRequireItems)
      (if (Utilities|Enum|Equal(Enum) _array_element_2 _array_element)
        (Utilities|Array|RemoveItem (Variables|Default|GetRequireItems) _array_element_2)
        (CallFunction|CEActiveChurchObjects _array_element)
        (Utilities|Array|RemoveItem (Variables|/Game/FirstPerson/Blueprints/BP_FirstPersonCharacter.BP_FirstPersonCharacter_C|GetInventario _returnvalue) _array_element)))
    (if (== (Utilities|Array|Length (Variables|Default|GetRequireItems)) 0)
      (Default|CallInteraction))))

(event EventTick
  (params (DeltaSeconds :type Float%20%28single-precision%29)))

(fn ConstructionScript)