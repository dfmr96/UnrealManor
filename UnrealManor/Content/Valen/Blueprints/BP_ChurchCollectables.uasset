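; BP_ChurchCollectables is a collectable item that registers itself with the first-person character's collection.
; Its CEAddObject custom event stores a self reference in ChurchCollectable, finds BP_FirstPersonCharacter via GetActorOfClass and passes ItemID to its FAddCollectable function.
; BeginPlay, overlap and Tick are disabled, and nothing in this graph calls CEAddObject.
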(event EventBeginPlay
  (|CallParentFunction) ; This node is disabled and will not be called.\nDrag off pins to build functionality.
)

(event Collision|EventActorBeginOverlap
  (params (OtherActor :type Actor%20Object%20Reference))
  (|CallParentFunction OtherActor) ; This node is disabled and will not be called.\nDrag off pins to build functionality.
)

(event EventTick
  (params (DeltaSeconds :type Float%20%28single-precision%29))
  (|CallParentFunction DeltaSeconds) ; This node is disabled and will not be called.\nDrag off pins to build functionality.
)

(event EventCEAddObject
  (Variables|Default|SetChurchCollectable self)
  (bind _returnvalue (Actor|GetActorOfClass "/Game/FirstPerson/Blueprints/BP_FirstPersonCharacter.BP_FirstPersonCharacter_C"))
  (Default|FAddCollectable _returnvalue (Variables|Default|GetItem_ID)))

(fn ConstructionScript
  (|CallParentFunction))