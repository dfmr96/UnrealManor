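; Tunnel pillar obstacle in the church level that slides open when BP_Altar fires its OpenPilaresTunel dispatcher.
; On BeginPlay it finds the altar and binds ABrirPilares, which runs once and plays a rock-moving sound.
; A Delay-driven loop, rather than a Timeline or Tick, nudges the two pillars in opposite local Y directions until the right one reaches its limit.
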(event Custom|ABrirPilares
  (bind _pilarderecho (Variables|Default|GetPilarDerecho))
  (Utilities|FlowControl|DoOnce false
    (:Completed
      (Audio|PlaySound2D "/Game/Audio/A_RockMoving.A_RockMoving" 1.0 1.0 0.0 0 0)
      (if (> (.y (Variables|/Script/Engine.SceneComponent|GetRelativeLocation _pilarderecho)) -237.0) :!label _label
        (Transformation|AddLocalOffset _pilarderecho "0.000000,-1.000000,0.000000" false false)
        (Transformation|AddLocalOffset (Variables|Default|GetPilarIzquierdo) "0.000000,1.000000,0.000000" false false)
        (Utilities|FlowControl|Delay 0.01)
        (goto _label)))))

(event EventBeginPlay
  (bind _returnvalue (Actor|GetActorOfClass "/Game/Blueprints/BP_Altar.BP_Altar_C"))
  (EventDispatchers|AssignOpenPilaresTunel _returnvalue (delegate Custom|ABrirPilares)))

(event Collision|EventActorBeginOverlap
  (params (OtherActor :type Actor%20Object%20Reference)))

(event EventTick
  (params (DeltaSeconds :type Float%20%28single-precision%29)))

(fn ConstructionScript)