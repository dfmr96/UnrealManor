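; BP_PaintLockV2 is a combination lock for the paint puzzle that opens a door when the correct digit sequence is received.
; ReceiveNumber appends each digit to TempCode and, once it matches the length of Code, compares the arrays element by element in order.
; A mismatch clears the entry and prints "Try Again".
; A match calls UnlockDoor, which uses a Timeline to move the Cube vertically by Height from its current relative location.
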(event Custom|ReceiveNumber
  (params (DigitValue :type Integer))
  (bind _tempcode (Variables|Default|GetTempCode))
  (bind _returnvalue (Utilities|Array|Length _tempcode))
  ;[1 1 1] Receive number and compare to "Code" array
  (Utilities|Array|Add _tempcode DigitValue)
  (Variables|Default|SetTempCodeIndex (- _returnvalue 1))
  (if (== _returnvalue (Utilities|Array|Length (Variables|Default|GetCode)))
    (for (_array_element _array_index) (Variables|Default|GetCode)
      (if (not (== _array_element (Utilities|Array|Get(acopy) (Variables|Default|GetTempCode) _array_index)))
        (Variables|Default|SetIncorrect true)))
    (if (Variables|Default|GetIncorrect)
      (Utilities|Array|Clear (Variables|Default|GetTempCode))
      (Variables|Default|SetTempCodeIndex 0)
      (Development|PrintString "Try Again")
      (Variables|Default|SetIncorrect false)
      (else
        (CallFunction|UnlockDoor)))))

(event Custom|UnlockDoor
  ;[1 1 1] Unlock Door
  (Variables|Default|SetCurrentLocation (Variables|/Script/Engine.SceneComponent|GetRelativeLocation (Variables|Default|GetCube)))
  (bind _position (Timeline|Timeline PlayFromStart)
    (:Update
      (Transformation|SetRelativeLocation (Variables|Default|GetCube) (+ (Variables|Default|GetCurrentLocation) (* _position (Math|Vector|MakeVector 0.0 0.0 (Variables|Default|GetHeight)))) false false))))

(fn ConstructionScript)