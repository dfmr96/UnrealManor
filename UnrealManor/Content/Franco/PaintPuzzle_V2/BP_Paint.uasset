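; BP_Paint is a paint piece in the paint puzzle, holding three child-actor BP_PaintButtonV2 buttons.
; On BeginPlay it gives each button its digit from the Paint1 array in ButtonValues and passes on its Lock reference.
; Interact sets the Box collision to BlockAll unless PaintLocked is set, and DisableCollision switches it to NoCollision.
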(event Custom|DisableCollision
  (Collision|SetCollisionProfileName (Variables|Default|GetBox) "NoCollision" true :!class /Script/Engine.PrimitiveComponent))

(event EventBeginPlay
  (for (_array_element _array_index) (Utilities|Array|MakeArray (Variables|Default|GetBP_PaintButtonV2) (Variables|Default|GetBP_PaintButtonV3) (Variables|Default|GetBP_PaintButtonV4))
    (bind _asbp_paint_button_v2 (Utilities|Casting|CastToBP_PaintButtonV2 (Variables|/Script/Engine.ChildActorComponent|GetChildActor _array_element)))
    (Variables|/Game/Franco/PaintPuzzle_V2/BP_PaintButtonV2.BP_PaintButtonV2_C|SetDigitValue _asbp_paint_button_v2 (Utilities|Array|Get(acopy) (Utilities|Struct|BreakBP_PaintButtonValues (Variables|Default|GetButtonValues)) _array_index))
    (Variables|/Game/Franco/PaintPuzzle_V2/BP_PaintButtonV2.BP_PaintButtonV2_C|SetLock _asbp_paint_button_v2 (Variables|Default|GetLock))))

(event EventInteract
  (if (not (Variables|Default|GetPaintLocked))
    (Collision|SetCollisionProfileName (Variables|Default|GetBox) "BlockAll" true :!class /Script/Engine.PrimitiveComponent)))

(fn ConstructionScript)