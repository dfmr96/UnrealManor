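; Nun enemy that prays idle until StopPraying, then reveals a knife and hunts the player.
; AIMoveTo drives a slow walk, then a faster chase once a sound finishes, retried on failure.
; ABP_Nun holds speed and state flags; a box overlap flags punch range and the hand collider deals damage.
; On death it stops moving, spawns a BP_CoreItem meshed from a data table, and disables the player's gun.
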(event OnComponentBeginOverlap(HandCollision)
  (params (OverlappedComponent :type Primitive%20Component%20Object%20Reference) (OtherActor :type Actor%20Object%20Reference) (OtherComp :type Primitive%20Component%20Object%20Reference) (OtherBodyIndex :type Integer) (bFromSweep :type Boolean) (SweepResult :type Hit%20Result%20Structure%20%28by%20ref%29))
  (if (not (Variables|/Game/Franco/Nun/anim/ABP_Nun.ABP_Nun_C|GetIsPraying (Variables|Default|GetNunAnim)))
    (if (not (Variables|/Game/Franco/Nun/anim/ABP_Nun.ABP_Nun_C|GetDeath (Variables|Default|GetNunAnim)))
      (if (== OtherActor (Variables|Default|GetPlayeref))
        (bind _asbp_first_person_character (Utilities|Casting|CastToBP_FirstPersonCharacter (Variables|Default|GetPlayeref)))
        (Default|TakeDamage _asbp_first_person_character (Variables|Default|GetDamage))))))

(event OnComponentBeginOverlap(Box)
  (params (OverlappedComponent :type Primitive%20Component%20Object%20Reference) (OtherActor :type Actor%20Object%20Reference) (OtherComp :type Primitive%20Component%20Object%20Reference) (OtherBodyIndex :type Integer) (bFromSweep :type Boolean) (SweepResult :type Hit%20Result%20Structure%20%28by%20ref%29))
  (if (not (Variables|/Game/Franco/Nun/anim/ABP_Nun.ABP_Nun_C|GetIsPraying (Variables|Default|GetNunAnim)))
    (if (== OtherActor (Variables|Default|GetPlayeref))
      (Variables|/Game/Franco/Nun/anim/ABP_Nun.ABP_Nun_C|SetEnemyAtPunchDistance (Variables|Default|GetNunAnim) true))))

(event OnComponentEndOverlap(Box)
  (params (OverlappedComponent :type Primitive%20Component%20Object%20Reference) (OtherActor :type Actor%20Object%20Reference) (OtherComp :type Primitive%20Component%20Object%20Reference) (OtherBodyIndex :type Integer))
  (bind _nunanim (Variables|Default|GetNunAnim))
  (if (not (Variables|/Game/Franco/Nun/anim/ABP_Nun.ABP_Nun_C|GetIsPraying (Variables|Default|GetNunAnim)))
    (if (== (Variables|Default|GetPlayeref) OtherActor)
      (Variables|/Game/Franco/Nun/anim/ABP_Nun.ABP_Nun_C|SetEnemyAtPunchDistance _nunanim false)
      (Variables|/Game/Franco/Nun/anim/ABP_Nun.ABP_Nun_C|SetSpeed _nunanim 0.0)
      (Transformation|SetRelativeLocation (Variables|Default|GetHandCollision) "0, 0, 0" false false)
      (Utilities|FlowControl|Delay 1.0)
      (CallFunction|ChasePlayer))))

(event Custom|StopPraying
  (Variables|/Game/Franco/Nun/anim/ABP_Nun.ABP_Nun_C|SetIsPraying (Variables|Default|GetNunAnim) false)
  (Audio|Components|Audio|Stop (Variables|Default|GetPrayerAudio))
  (CallFunction|WalktoPlayers))

(event Custom|ChasePlayer
  (bind _self self)
  (bind _playeref (Variables|Default|GetPlayeref))
  (bind _nunanim (Variables|Default|GetNunAnim))
  (bind _nunanim_2 (Variables|Default|GetNunAnim))
  (bind _death (Variables|/Game/Franco/Nun/anim/ABP_Nun.ABP_Nun_C|GetDeath _nunanim_2))
  (bind _death_2 (Variables|/Game/Franco/Nun/anim/ABP_Nun.ABP_Nun_C|GetDeath _nunanim))
  (bind _charactermovement (Variables|Character|GetCharacterMovement _self))
  (Utilities|FlowControl|Sequence
    (:then_0
      (Utilities|IsValid (Variables|Default|GetPlayeref)
        (:Is%20Valid
          (if (not _death)
            (Variables|/Game/Franco/Nun/anim/ABP_Nun.ABP_Nun_C|SetSpeed _nunanim_2 1e+02)
            (AI|AIMoveTo self (Transformation|GetWorldLocation (Variables|/Script/Engine.Character|GetCapsuleComponent _playeref)) _playeref 1e+01 _death
              (:then
                (if _death_2
                  (Pawn|Components|CharacterMovement|DisableMovement (Variables|Character|GetCharacterMovement))))
              (:OnFail
                (if (not _death_2)
                  (CallFunction|ChasePlayer))))))))
    (:then_1
      (Utilities|FlowControl|DoOnce false
        (:Completed
          (Variables|/Script/Engine.CharacterMovementComponent|SetMaxWalkSpeed _charactermovement (* (Variables|/Script/Engine.CharacterMovementComponent|GetMaxWalkSpeed _charactermovement) 2.0)))))))

(event Custom|WalkToPlayers
  (bind _self self)
  (bind _nunanim (Variables|Default|GetNunAnim))
  (bind _sound (Variables|Default|GetSound))
  (bind _playeref (Variables|Default|GetPlayeref))
  (bind _death (Variables|/Game/Franco/Nun/anim/ABP_Nun.ABP_Nun_C|GetDeath _nunanim))
  (bind _charactermovement (Variables|Character|GetCharacterMovement _self))
  (Development|SetHiddeninGame (Variables|Default|GetKnife) false false)
  (Variables|/Script/Engine.CharacterMovementComponent|SetMaxWalkSpeed _charactermovement (/ (Variables|/Script/Engine.CharacterMovementComponent|GetMaxWalkSpeed _charactermovement) 2.0))
  (Utilities|IsValid (Variables|Default|GetPlayeref)
    (:Is%20Valid
      (if (not _death)
        (Variables|/Game/Franco/Nun/anim/ABP_Nun.ABP_Nun_C|SetSpeed _nunanim 49.0)
        (AI|AIMoveTo self (Transformation|GetWorldLocation (Variables|/Script/Engine.Character|GetCapsuleComponent _playeref)) _playeref 1e+01 _death
          (:then
            (Audio|PlaySound2D _sound 1.0 1.0 0.0 0 0 false)
            (Utilities|FlowControl|Delay (Variables|/Script/Engine.SoundBase|GetDuration _sound))
            (CallFunction|ChasePlayer)))))))

(event EventBeginPlay
  (Development|SetHiddeninGame (Variables|Default|GetKnife) true false)
  (Variables|Default|SetPlayeref (Game|GetPlayerCharacter 0))
  (bind _asabp_nun (Utilities|Casting|CastToABP_Nun (Components|SkeletalMesh|GetAnimInstance (Variables|Character|GetMesh))))
  (bind _output_get (Variables|Default|SetNunAnim _asabp_nun))
  (Variables|/Game/Franco/Nun/anim/ABP_Nun.ABP_Nun_C|SetSpeed _output_get 0.0)
  (Variables|/Game/Franco/Nun/anim/ABP_Nun.ABP_Nun_C|SetIsPraying (Variables|Default|GetNunAnim) true))

(event EventTakeDamage
  (params (Damage :type Integer))
  (bind _capsulecomponent (Variables|Collision|GetCapsuleComponent))
  (if (> (Variables|Default|Gethealth) 0.0)
    (bind _output_get (Variables|Default|Sethealth (- (Variables|Default|Gethealth) Damage)))
    (Development|PrintString (Utilities|String|Append "Enemy damaged. Current health: " (Utilities|String|ToString(Integer) (Math|Float|Truncate _output_get))))
    (if (<= _output_get 0)
      (Development|PrintString "Enemy destroyed")
      (Variables|/Game/Franco/Nun/anim/ABP_Nun.ABP_Nun_C|SetDeath (Variables|Default|GetNunAnim) true)
      (Pawn|Components|CharacterMovement|DisableMovement (Variables|Character|GetCharacterMovement))
      (bind _returnvalue (Game|SpawnActorfromClass "/Game/Blueprints/Inventory/ItemClasses/BP_CoreItem.BP_CoreItem_C" (Math|Conversions|ToTransform(Vector) (Transformation|GetWorldLocation (Variables|Character|GetMesh))) "Undefined" "MultiplyWithRoot" 0 0))
      (Collision|SetCollisionResponsetoChannel _capsulecomponent "ECC_Visibility" "ECR_Ignore")
      (Collision|SetCollisionResponsetoChannel _capsulecomponent "ECC_Camera" "ECR_Ignore")
      (bind _output_get_2 (Variables|/Game/Blueprints/Inventory/ItemClasses/BP_GroundItem.BP_GroundItem_C|SetItemData _returnvalue (Variables|Default|GetItem%20Data)))
      (bind _returnvalue_2 (Utilities|GetDataTableRow "/Game/Blueprints/Inventory/ItemDataTable.ItemDataTable" (.rowname _output_get_2))
        (:then
          (Components|StaticMesh|SetStaticMesh (Variables|/Game/Blueprints/Inventory/ItemClasses/BP_GroundItem.BP_GroundItem_C|GetBody _returnvalue) (.mesh _returnvalue_2))
          (bind _asbp_first_person_character (Utilities|Casting|CastToBP_FirstPersonCharacter (Variables|Default|GetPlayeref) :!label _label)
            (:then
              (Default|DisableGun _asbp_first_person_character))
            (:CastFailed
              (Utilities|FlowControl|Delay 0.2)
              (goto _label))))))))

(fn ConstructionScript)