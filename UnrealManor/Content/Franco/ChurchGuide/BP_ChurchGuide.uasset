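; BP_ChurchGuide is an interactable readable church guide that opens and closes a text widget.
; Interact toggles on IsOpen, playing a page-turning sound and creating or removing the TextWidget.
; While open, player movement and look input are disabled, input switches to game-and-UI, and the character's FileWidget reference is cleared.
; Closing restores walking and game-only input, then triggers garbage collection.
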(event EventInteract
  (bind _returnvalue (Game|GetPlayerController 0))
  (if (Variables|Default|GetisOpen)
    (Audio|PlaySound2D "/Game/Audio/Objects__Book__Document__Thick__Many_Pages__Search_Through__Find_Page_SND17731_4.Objects__Book__Document__Thick__Many_Pages__Search_Through__Find_Page_SND17731_4" 1.0 1.0 0.0 0 0)
    (Widget|SetVisibility (Variables|Default|GetnewWidget) "Hidden")
    (Widget|RemovefromParent (Variables|Default|GetnewWidget))
    (Utilities|Platform|CollectGarbage)
    (Input|SetInputModeGameOnly (Game|GetPlayerController 0) false)
    (Variables|Default|SetisOpen false)
    (Pawn|Components|CharacterMovement|SetMovementMode (Variables|/Script/Engine.Character|GetCharacterMovement (Game|GetPlayerCharacter 0)) "MOVE_Walking" 0)
    (Input|SetIgnoreLookInput (Game|GetPlayerController 0) false)
    (else
      (Audio|PlaySound2D "/Game/Audio/Objects__Book__Document__Thick__Many_Pages__Search_Through__Find_Page_SND17731_2.Objects__Book__Document__Thick__Many_Pages__Search_Through__Find_Page_SND17731_2" 1.0 1.0 0.0 0 0)
      (Pawn|Components|CharacterMovement|DisableMovement (Variables|/Script/Engine.Character|GetCharacterMovement (Game|GetPlayerCharacter 0)))
      (bind _returnvalue_2 (UserInterface|CreateWidget (Variables|Default|GetTextWidget)))
      (bind _output_get (Variables|Default|SetnewWidget _returnvalue_2))
      (Variables|/Game/Core/FirstPerson/Blueprints/BP_FirstPersonCharacter.BP_FirstPersonCharacter_C|SetFileWidget (.AsBP%20First%20Person%20Character (Utilities|Casting|CastToBP_FirstPersonCharacter (Game|GetPlayerCharacter 0))) 0)
      (Widget|SetVisibility _output_get "Visible")
      (UserInterface|Viewport|AddtoViewport (Variables|Default|GetnewWidget) 0)
      (Input|SetIgnoreLookInput _returnvalue true)
      (Input|SetInputModeGameandUI (.AsBP%20First%20Person%20Player%20Controller (Utilities|Casting|CastToBP_FirstPersonPlayerController _returnvalue)) (Variables|Default|GetnewWidget) "LockOnCapture" true false)
      (Variables|Default|SetisOpen true))))

(fn ConstructionScript)