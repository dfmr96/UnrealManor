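; BP_RatTrigger is a one-shot trigger that sets a group of rats moving when the player walks into it.
; On player overlap, it plays a mouse footsteps sound at its own location, then loops over its Rat array, calling Move with FowardMultiplier and playing an attenuated squeak at each rat.
; The trigger then destroys itself, so the event cannot repeat.
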(event OnComponentBeginOverlap(Trigger)
  (params (OverlappedComponent :type Primitive%20Component%20Object%20Reference) (OtherActor :type Actor%20Object%20Reference) (OtherComp :type Primitive%20Component%20Object%20Reference) (OtherBodyIndex :type Integer) (bFromSweep :type Boolean) (SweepResult :type Hit%20Result%20Structure%20%28by%20ref%29))
  (if (== OtherActor (Game|GetPlayerCharacter 0))
    (Audio|PlaySoundatLocation "/Game/Franco/Rat/A_MouseSteps.A_MouseSteps" (Transformation|GetActorLocation self) "0, 0, 0" 0.5 1.0 0.0 "/Game/Audio/SA_Prayer.SA_Prayer" 0 0 0)
    (for _array_element (Variables|Default|GetRat)
      (Default|Move _array_element (Variables|Default|GetFowardMultiplier))
      (Audio|PlaySoundatLocation "/Game/Franco/Rat/A_MouseSqueak.A_MouseSqueak" (Transformation|GetActorLocation _array_element) "0, 0, 0" 0.75 1.0 4.0 "/Game/Audio/SA_Prayer.SA_Prayer" 0 0 0))
    (Actor|DestroyActor)))

(fn ConstructionScript)