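; BP_Rosary is a single-use interactable rosary that relieves the player's curse effects and destroys itself when used.
; Interact reads the PC_Data_PP material parameter collection, lowering Blindness by a fixed step while it is above a small threshold.
; Otherwise it lowers Alpha by CurseHealing, with both values clamped to the zero-to-one range.
; When FirstRosary is set, it also plays a 2D sound after the destroy call.
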(event EventInteract
  (bind _returnvalue (Rendering|Material|GetScalarParameterValue "/Game/Franco/Materiales_PostProccess/PC_Data_PP.PC_Data_PP" "Blindness" :!class /Script/Engine.KismetMaterialLibrary))
  (if (> _returnvalue 0.1)
    (Rendering|Material|SetScalarParameterValue "/Game/Franco/Materiales_PostProccess/PC_Data_PP.PC_Data_PP" "Blindness" (Math|Float|Clamp(Float) (- _returnvalue 0.2)) :!class /Script/Engine.KismetMaterialLibrary)
    (else
      (bind _returnvalue_2 (Rendering|Material|GetScalarParameterValue "/Game/Franco/Materiales_PostProccess/PC_Data_PP.PC_Data_PP" "Alpha" :!class /Script/Engine.KismetMaterialLibrary))
      (Rendering|Material|SetScalarParameterValue "/Game/Franco/Materiales_PostProccess/PC_Data_PP.PC_Data_PP" "Alpha" (Math|Float|Clamp(Float) (- _returnvalue_2 (Variables|Default|GetCurseHealing))) :!class /Script/Engine.KismetMaterialLibrary)))
  (Actor|DestroyActor)
  (if (Variables|Default|GetFirstRosary?)
    (Audio|PlaySound2D (Variables|Default|GetSFX) 1.0 1.0 0.0 0 0)))

(fn ConstructionScript)