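; BP_RomeroWindow is a breakable window that spawns a BP_Romero character when TriggerWindow is called.
; Romero spawns at the Arrow's transform, receives the window's Health and Damage, stands up and gets a reference to the player.
; The glass Geometry Collection then starts simulating physics with a sound, as its PhysicsObstacle is destroyed and the glass's collision is disabled.
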(event Custom|BreakGlass
  (Physics|SetSimulatePhysics (Variables|Default|GetSM_Glass_GeometryCollection) true)
  (Audio|PlaySoundatLocation (Variables|Default|GetSFX) (Transformation|GetWorldLocation (Variables|Default|GetPhysicsObstacle)) "0, 0, 0" 1.0 1.0 0.0 0 0 0 0)
  (Components|DestroyComponent (Variables|Default|GetPhysicsObstacle)))

(event Custom|TriggerWindow
  (CallFunction|SpawnRomero)
  (CallFunction|BreakGlass)
  (Collision|SetCollisionEnabled (Variables|Default|GetSM_Glass_GeometryCollection) "NoCollision"))

(event Custom|SpawnRomero
  (bind _arrow (Variables|Default|GetArrow))
  (bind _returnvalue (Game|SpawnActorfromClass "/Game/Franco/Romero/BP_Romero.BP_Romero_C" (Math|Transform|MakeTransform (Transformation|GetWorldLocation _arrow) (Transformation|GetWorldRotation _arrow) "1.000000,1.000000,1.000000") "AdjustIfPossibleButAlwaysSpawn" "MultiplyWithRoot" 0 0))
  (bind _output_get (Variables|Default|SetRomero _returnvalue))
  (Variables|/Game/Franco/Romero/BP_Romero.BP_Romero_C|SetHealth _output_get (Variables|Default|GetHealth))
  (Variables|/Game/Franco/Romero/BP_Romero.BP_Romero_C|SetDamage (Variables|Default|GetRomero) (Variables|Default|GetDamage))
  (Default|StandUp (Variables|Default|GetRomero))
  (Variables|/Game/Franco/Romero/BP_Romero.BP_Romero_C|SetPlayeref (Variables|Default|GetRomero) (Game|GetPlayerCharacter 0)))

(fn ConstructionScript)