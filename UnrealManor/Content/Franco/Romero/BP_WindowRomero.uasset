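; Window ambush actor that, on TriggerBP, spawns a BP_Romero enemy and shatters its glass.
; The enemy spawns at the Arrow component's transform, receives this actor's Health and Damage, then calls StandUp.
; The glass break enables physics on a Geometry Collection and plays a 2D sound.
; TriggerBP checks AlreadyTriggered, but this graph never sets that flag.
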(event Custom|TriggerBP
  (if (not (Variables|Default|GetAlreadyTriggered))
    (CallFunction|SpawnEnemy)
    (CallFunction|BreakGlass)))

(event Custom|SpawnEnemy
  (bind _arrow (Variables|Default|GetArrow))
  (bind _returnvalue (Game|SpawnActorfromClass "/Game/Franco/Romero/BP_Romero.BP_Romero_C" (Math|Transform|MakeTransform (Transformation|GetWorldLocation _arrow) (Transformation|GetWorldRotation _arrow) "1.000000,1.000000,1.000000") "AdjustIfPossibleButAlwaysSpawn" "MultiplyWithRoot" 0 0))
  (Variables|/Game/Franco/Romero/BP_Romero.BP_Romero_C|SetHealth _returnvalue (Variables|Default|GetHealth))
  (Variables|/Game/Franco/Romero/BP_Romero.BP_Romero_C|SetDamage _returnvalue (Variables|Default|GetDamage))
  (Default|StandUp _returnvalue))

(event Custom|BreakGlass
  (Physics|SetSimulatePhysics (Variables|Default|GetSM_Glass_GeometryCollection) true)
  (Audio|PlaySound2D (Variables|Default|GetSFX) 1.0 1.0 0.0 0 0))

(fn ConstructionScript)