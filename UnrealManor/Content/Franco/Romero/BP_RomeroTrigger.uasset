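; BP_RomeroTrigger is a one-shot gaze trigger that calls TriggerWindow on an array of Glass objects.
; BeginLooked adds DeltaSeconds to a counter and fires once it reaches WaitingTime.
; Below that threshold, a Delay of WaitingTime plus one second zeroes the counter if still untriggered, timed from the call that started it rather than from when looking stops.
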(event EventBeginLooked
  (params (DeltaSeconds :type Float%20%28double-precision%29))
  (if (not (Variables|Default|GetTriggerActivated))
    (Variables|Default|SetCounter (+ DeltaSeconds (Variables|Default|GetCounter)))
    (if (>= (Variables|Default|GetCounter) (Variables|Default|GetWaitingTime))
      (Variables|Default|SetTriggerActivated true)
      (for _array_element (Variables|Default|GetGlass)
        (Default|TriggerWindow _array_element))
      (else
        (Utilities|FlowControl|Delay (+ (Variables|Default|GetWaitingTime) 1.0))
        (if (not (Variables|Default|GetTriggerActivated))
          (Development|PrintString "TimerReset")
          (Variables|Default|SetCounter 0.0))))))

(fn ConstructionScript)