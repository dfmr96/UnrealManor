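; BP_Romero is a melee enemy character that stands up shortly after spawning, then idles.
; ChasePlayer re-issues AI MoveTo on the player in a loop; within the file, only leaving the punch-range box starts it.
; It drives ABP_Romero variables for speed, punching and death, while hand-collision overlaps damage the player.
; TakeDamage lowers health and, at zero, flags death and disables collision.
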(event OnComponentBeginOverlap(HandCollision)
  (params (OverlappedComponent :type Primitive%20Component%20Object%20Reference) (OtherActor :type Actor%20Object%20Reference) (OtherComp :type Primitive%20Component%20Object%20Reference) (OtherBodyIndex :type Integer) (bFromSweep :type Boolean) (SweepResult :type Hit%20Result%20Structure%20%28by%20ref%29))
  (if (not (Variables|/Game/Franco/Romero/Animations/ABP_Romero.ABP_Romero_C|GetDeath (Variables|Default|GetRomeroAnim)))
    (if (== OtherActor (Variables|Default|GetPlayeref))
      (bind _asbp_first_person_character (Utilities|Casting|CastToBP_FirstPersonCharacter (Variables|Default|GetPlayeref)))
      (Default|TakeDamage _asbp_first_person_character (Variables|Default|GetDamage)))))

(event OnComponentBeginOverlap(Box)
  (params (OverlappedComponent :type Primitive%20Component%20Object%20Reference) (OtherActor :type Actor%20Object%20Reference) (OtherComp :type Primitive%20Component%20Object%20Reference) (OtherBodyIndex :type Integer) (bFromSweep :type Boolean) (SweepResult :type Hit%20Result%20Structure%20%28by%20ref%29))
  (if (== OtherActor (Variables|Default|GetPlayeref))
    (Variables|/Game/Franco/Romero/Animations/ABP_Romero.ABP_Romero_C|SetEnemyAtPunchDistance (Variables|Default|GetRomeroAnim) true)))

(event OnComponentEndOverlap(Box)
  (params (OverlappedComponent :type Primitive%20Component%20Object%20Reference) (OtherActor :type Actor%20Object%20Reference) (OtherComp :type Primitive%20Component%20Object%20Reference) (OtherBodyIndex :type Integer))
  (bind _romeroanim (Variables|Default|GetRomeroAnim))
  (if (== (Variables|Default|GetPlayeref) OtherActor)
    (Variables|/Game/Franco/Romero/Animations/ABP_Romero.ABP_Romero_C|SetEnemyAtPunchDistance _romeroanim false)
    (Variables|/Game/Franco/Romero/Animations/ABP_Romero.ABP_Romero_C|SetSpeed _romeroanim 0.0)
    (Transformation|SetRelativeLocation (Variables|Default|GetHandCollision) "0, 0, 0" false false)
    (Utilities|FlowControl|Delay 1.0)
    (CallFunction|ChasePlayer)))

(event Custom|StandUp
  (Variables|/Game/Franco/Romero/Animations/ABP_Romero.ABP_Romero_C|SetStandUp (Variables|Default|GetRomeroAnim) true)
  (CallFunction|Idle))

(event Custom|ChasePlayer
  (bind _romeroanim (Variables|Default|GetRomeroAnim))
  (bind _playeref (Variables|Default|GetPlayeref))
  (Utilities|IsValid (Variables|Default|GetPlayeref)
    (:Is%20Valid
      (if (not (Variables|/Game/Franco/Romero/Animations/ABP_Romero.ABP_Romero_C|GetDeath _romeroanim))
        (Variables|/Game/Franco/Romero/Animations/ABP_Romero.ABP_Romero_C|SetSpeed _romeroanim 1e+02)
        (AI|AIMoveTo self (Transformation|GetWorldLocation (Variables|/Script/Engine.Character|GetCapsuleComponent _playeref)) _playeref 1.0 false
          (:OnSuccess
            _)
          (:OnFail
            _))
        (Utilities|FlowControl|Delay 0.5)
        (CallFunction|ChasePlayer)))))

(event Custom|Idle
  (bind _romeroanim (Variables|Default|GetRomeroAnim))
  (if (not (Variables|/Game/Franco/Romero/Animations/ABP_Romero.ABP_Romero_C|GetIdle (Variables|Default|GetRomeroAnim)))
    (Variables|/Game/Franco/Romero/Animations/ABP_Romero.ABP_Romero_C|SetIdle _romeroanim true)
    (Variables|/Game/Franco/Romero/Animations/ABP_Romero.ABP_Romero_C|SetSpeed _romeroanim 0.0)))

(event EventBeginPlay
  (Variables|Default|SetPlayeref (Game|GetPlayerCharacter 0))
  (bind _asabp_romero (Utilities|Casting|CastToABP_Romero (Components|SkeletalMesh|GetAnimInstance (Variables|Character|GetMesh)) :!label _label)
    (:then
      (Variables|Default|SetRomeroAnim _asabp_romero)
      (Utilities|FlowControl|Delay 3.0)
      (CallFunction|StandUp))
    (:CastFailed
      (Utilities|FlowControl|Delay 0.2)
      (goto _label))))

(event EventTakeDamage
  (params (Damage :type Integer))
  (if (> (Variables|Default|Gethealth) 0.0)
    (bind _output_get (Variables|Default|Sethealth (- (Variables|Default|Gethealth) Damage)))
    (Development|PrintString (Utilities|String|Append "Enemy damaged. Current health: " (Utilities|String|ToString(Integer) (Math|Float|Truncate _output_get))))
    (if (<= _output_get 0)
      (Development|PrintString "Enemy destroyed")
      (Variables|/Game/Franco/Romero/Animations/ABP_Romero.ABP_Romero_C|SetDeath (Variables|Default|GetRomeroAnim) true)
      (Collision|SetActorEnableCollision self false))))

(fn ConstructionScript)