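; BP_ResetChessPieces is a trigger volume that resets the pieces of a chess puzzle to their starting positions.
; Shortly after BeginPlay it caches the location of every actor in its Actor array.
; When the player character overlaps the Box, it moves each actor back to its cached location by index, unless ChessPuzzle reports the puzzle completed.
; An unconnected leftover branch holds single-actor reset logic with destroy and sound handling.
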(event OnComponentBeginOverlap(Box)
  (params (OverlappedComponent :type Primitive%20Component%20Object%20Reference) (OtherActor :type Actor%20Object%20Reference) (OtherComp :type Primitive%20Component%20Object%20Reference) (OtherBodyIndex :type Integer) (bFromSweep :type Boolean) (SweepResult :type Hit%20Result%20Structure%20%28by%20ref%29))
  (if (not (Variables|/Game/Blueprints/Puzzles/Chess/BP_ChessPuzzle.BP_ChessPuzzle_C|GetPuzzleCompleted (Variables|Default|GetChessPuzzle)))
    (if (== OtherActor (Game|GetPlayerCharacter 0))
      (for (_array_element _array_index) (Variables|Default|GetActor)
        (Transformation|SetActorLocation _array_element (Utilities|Array|Get(acopy) (Variables|Default|GetActorOriginalLocation) _array_index) false false)))))

(event EventBeginPlay
  (Utilities|FlowControl|Delay 0.2)
  (for _array_element (Variables|Default|GetActor)
    (Utilities|Array|Add (Variables|Default|GetActorOriginalLocation) (Transformation|GetActorLocation _array_element))))

(fn ConstructionScript)