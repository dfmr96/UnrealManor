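; BP_ResetLocation is a trigger that resets a referenced pushable object to its starting position when the player enters its box.
; It caches that actor's location shortly after BeginPlay, then on overlap teleports it back with a sound if it has moved.
; If the actor, cast to BP_PushableObjectDrop, is Broken, the trigger instead destroys an optional DestroyActor and itself.
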(event OnComponentBeginOverlap(Box)
  (params (OverlappedComponent :type Primitive%20Component%20Object%20Reference) (OtherActor :type Actor%20Object%20Reference) (OtherComp :type Primitive%20Component%20Object%20Reference) (OtherBodyIndex :type Integer) (bFromSweep :type Boolean) (SweepResult :type Hit%20Result%20Structure%20%28by%20ref%29))
  (bind _destroyactor (Variables|Default|GetDestroyActor))
  (if (== OtherActor (Game|GetPlayerCharacter 0))
    (bind _asbp_pushable_object_drop (Utilities|Casting|CastToBP_PushableObjectDrop (Variables|Default|GetActor)))
    (if (Variables|/Game/Franco/PushableStatue/BP_PushableObjectDrop.BP_PushableObjectDrop_C|GetBroken _asbp_pushable_object_drop)
      (Utilities|IsValid _destroyactor
        (:Is%20Valid
          (Actor|DestroyActor _destroyactor))
        (:Is%20Not%20Valid
          _))
      (Actor|DestroyActor)
      (elif (not (Utilities|Operators|EqualEqual (Transformation|GetActorLocation (Variables|Default|GetActor)) (Variables|Default|GetActorOriginalLocation) 0.0))
        (Transformation|SetActorLocation (Variables|Default|GetActor) (Variables|Default|GetActorOriginalLocation) false true)
        (Audio|PlaySoundatLocation (Variables|Default|GetSound) (Variables|Default|GetActorOriginalLocation) "0, 0, 0" 1.0 1.0 0.0 0 0 0 0)))))

(event EventBeginPlay
  (Utilities|FlowControl|Delay 0.2)
  (Variables|Default|SetActorOriginalLocation (Transformation|GetActorLocation (Variables|Default|GetActor))))

(fn ConstructionScript)