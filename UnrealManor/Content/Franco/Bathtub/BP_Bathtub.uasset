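; Bathtub actor that drains its water, with a sound effect, when its Drain event is called.
; On BeginPlay it registers itself with its Plug through a Bathtub reference.
; Drain plays a timeline that lowers the Water component cumulatively by the Movement track each update.
; An Empty flag blocks further lowering, set only when the water's relative location exactly matches a hardcoded bottom position.
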(event Custom|Drain
  (bind _water (Variables|Default|GetWater))
  (Audio|PlaySound2D "/Game/Audio/A_BathDraining.A_BathDraining" 1.0 1.0 0.0 0 0)
  (Variables|Default|SetPlaneLocation (Transformation|GetWorldLocation (Variables|Default|GetWater)))
  (if (not (Variables|Default|GetEmpty?))
    (Timeline|Timeline PlayFromStart
      (:Update
        (Transformation|SetWorldLocation (Variables|Default|GetWater) (- (Variables|Default|GetPlaneLocation) (Math|Vector|MakeVector 0.0 0.0 (Variables|Default|GetMovement))) false false)
        (Variables|Default|SetPlaneLocation (Transformation|GetWorldLocation _water))
        (if (Utilities|Operators|EqualEqual (Variables|/Script/Engine.SceneComponent|GetRelativeLocation _water) "-1.893600,-1.102113,-19.000000" 0.0)
          (Variables|Default|SetEmpty? true))))))

(event EventBeginPlay
  (Variables|/Game/Franco/Bathtub/BP_Plug.BP_Plug_C|SetBathtub (Variables|Default|GetPlug) self))

(fn ConstructionScript)