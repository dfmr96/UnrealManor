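; One-shot trigger actor that plays a sound, by its name glass cracking, when the player enters its Box.
; The first overlap by player character 0 plays SFX at the Audio component's location and sets AlreadyCracked to block repeats.
; The actor then waits for the sound's duration and destroys itself.
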(event OnComponentBeginOverlap(Box)
  (params (OverlappedComponent :type Primitive%20Component%20Object%20Reference) (OtherActor :type Actor%20Object%20Reference) (OtherComp :type Primitive%20Component%20Object%20Reference) (OtherBodyIndex :type Integer) (bFromSweep :type Boolean) (SweepResult :type Hit%20Result%20Structure%20%28by%20ref%29))
  (if (not (Variables|Default|GetAlreadyCracked))
    (if (== OtherActor (Game|GetPlayerCharacter 0))
      (Utilities|FlowControl|Sequence
        (:then_0
          (Audio|PlaySoundatLocation (Variables|Default|GetSFX) (Transformation|GetWorldLocation (Variables|Default|GetAudio)) "0, 0, 0" 1.0 1.0 0.0 0 0 0 0)
          (Variables|Default|SetAlreadyCracked true))
        (:then_1
          (Utilities|FlowControl|Delay (Variables|/Script/Engine.SoundBase|GetDuration (Variables|Default|GetSFX)))
          (Actor|DestroyActor))))))

(fn ConstructionScript)