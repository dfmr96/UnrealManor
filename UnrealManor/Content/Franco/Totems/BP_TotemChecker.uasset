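; BP_TotemChecker is an interactable gate check that decides whether the final door unlocks based on burnt totems.
; On Interact it counts entries in its Totems array with IsBurnt set, then sets FinalEnabled when the count equals the array length.
; The door result is only printed as a debug string here.
; TotemsDestroyed is never reset in this graph, so the count accumulates across repeated interactions.
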(event EventInteract
  (for _array_element (Variables|Default|GetTotems)
    (if (Variables|/Game/Blueprints/BP_Totems.BP_Totems_C|GetisBurnt? _array_element)
      (Variables|Default|SetTotemsDestroyed (+ 1 (Variables|Default|GetTotemsDestroyed)))))
  (if (== (Utilities|Array|Length (Variables|Default|GetTotems)) (Variables|Default|GetTotemsDestroyed))
    (Development|PrintString "UnlockDoor")
    (Variables|Default|SetFinalEnabled true)
    (else
      (Development|PrintString "DoorLocked")
      (Variables|Default|SetFinalEnabled false))))

(fn ConstructionScript)