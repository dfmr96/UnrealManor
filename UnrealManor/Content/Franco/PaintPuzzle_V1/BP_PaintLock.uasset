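; BP_PaintLock is a puzzle lock that opens a door when its buttons send digits in the correct order.
; On BeginPlay it shuffles Buttons and Code, then gives each button a digit and a matching mesh from a MeshMap lookup.
; ReceiveNumber checks each digit against the code sequence, resetting progress on a mistake.
; Completing the sequence triggers UnlockDoor, where a Timeline moves the Cube along Z by Height.
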(event Custom|ReceiveNumber
  (params (DigitValue :type Integer))
  ;[1 1 1] Receive number and compare to "Code" array
  (if (== DigitValue (Utilities|Array|Get(acopy) (Variables|Default|GetCode) (Variables|Default|GetCodeIndex)))
    (if (== (Variables|Default|GetCodeIndex) (- (Utilities|Array|Length (Variables|Default|GetCode)) 1))
      (CallFunction|UnlockDoor)
      (else
        (Variables|Default|SetCodeIndex (+ (Variables|Default|GetCodeIndex) 1))))
    (else
      (Variables|Default|SetCodeIndex 0)
      (Development|PrintString "WrongNumber"))))

(event Custom|UnlockDoor
  ;[1 1 1] Unlock Door
  (Variables|Default|SetCurrentLocation (Variables|/Script/Engine.SceneComponent|GetRelativeLocation (Variables|Default|GetCube)))
  (bind _position (Timeline|Timeline PlayFromStart)
    (:Update
      (Transformation|SetRelativeLocation (Variables|Default|GetCube) (+ (Variables|Default|GetCurrentLocation) (* _position (Math|Vector|MakeVector 0.0 0.0 (Variables|Default|GetHeight)))) false false))))

(event EventBeginPlay
  (bind _code (Variables|Default|GetCode))
  ;[1 1 1] Assing a digit value and mesh to each button
  (Utilities|Array|Shuffle (Variables|Default|GetButtons))
  (Utilities|Array|Shuffle _code)
  (for (_array_element _array_index) _code
    (bind _output_get (Variables|/Game/Franco/PaintPuzzle_V1/BP_PaintButton.BP_PaintButton_C|SetDigitValue (Utilities|Array|Get(acopy) (Variables|Default|GetButtons) _array_index) _array_element))
    (Development|PrintString (Utilities|String|ToString(Integer) _output_get) true true "(R=0.000000,G=0.660000,B=1.000000,A=1.000000)" 1e+01)
    (Components|StaticMesh|SetStaticMesh (Variables|/Game/Franco/PaintPuzzle_V1/BP_PaintButton.BP_PaintButton_C|GetCube (Utilities|Array|Get(acopy) (Variables|Default|GetButtons) _array_index)) (.Value (Utilities|Map|Find (Utilities|Struct|BreakPaintCollections (Variables|Default|GetMesh)) _output_get)))))

(fn ConstructionScript)